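; Floor button that activates linked steles and raises a linked door when stepped on, with its label set in the construction script.
; BeginPlay clears the steles' button-activation flag; any actor entering the box sets it, looping over the array.
; The player-only door move runs inside that loop, using MoveComponentTo with world-space transforms as relative targets.
; Exiting lowers the door (marked untested); unreset DoOnce gates limit each move to once.
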(event OnComponentBeginOverlap(Box)
  (params (OverlappedComponent :type Primitive%20Component%20Object%20Reference) (OtherActor :type Actor%20Object%20Reference) (OtherComp :type Primitive%20Component%20Object%20Reference) (OtherBodyIndex :type Integer) (bFromSweep :type Boolean) (SweepResult :type Hit%20Result%20Structure%20%28by%20ref%29))
  (bind _bp_doortoopen (Variables|Default|GetBP_DoorToOpen))
  (bind _petite_porte_mobile (Variables|/Game/Blueprints/BP_Door/BP_Door.BP_Door_C|GetPetite_Porte_Mobile _bp_doortoopen))
  (bind _returnvalue (Transformation|GetWorldLocation _petite_porte_mobile))
  (for _array_element (Variables|Default|GetBP_SteleToActivate)
    (Variables|/Game/Blueprints/BP_Steles/BP_StelesMother.BP_StelesMother_C|SetIsActivateByLevelButton _array_element true)
    (Utilities|Casting|CastToBP_PlayerProto OtherActor)
    (Utilities|FlowControl|DoOnce false
      (:Completed
        (Utilities|IsValid (Variables|Default|GetBP_DoorToOpen)
          (:Is%20Valid
            (Components|MoveComponentTo _petite_porte_mobile (Math|Vector|MakeVector (.x _returnvalue) (.y _returnvalue) (+ (.z _returnvalue) 3e+02)) (Transformation|GetWorldRotation _petite_porte_mobile) false false (Variables|/Game/Blueprints/BP_Door/BP_Door.BP_Door_C|GetOpeningDoorTime _bp_doortoopen) false)))))))

(event OnComponentEndOverlap(Box)
  (params (OverlappedComponent :type Primitive%20Component%20Object%20Reference) (OtherActor :type Actor%20Object%20Reference) (OtherComp :type Primitive%20Component%20Object%20Reference) (OtherBodyIndex :type Integer))
  (bind _bp_doortoopen (Variables|Default|GetBP_DoorToOpen))
  (bind _petite_porte_mobile (Variables|/Game/Blueprints/BP_Door/BP_Door.BP_Door_C|GetPetite_Porte_Mobile _bp_doortoopen))
  (bind _returnvalue (Transformation|GetWorldLocation _petite_porte_mobile))
  ;[1 1 1] Doit refermer la porte quand on sort de la box - A TESTER
  (Utilities|Casting|CastToBP_PlayerProto OtherActor)
  (Utilities|FlowControl|DoOnce false
    (:Completed
      (Utilities|IsValid (Variables|Default|GetBP_DoorToOpen)
        (:Is%20Valid
          (Components|MoveComponentTo _petite_porte_mobile (Math|Vector|MakeVector (.x _returnvalue) (.y _returnvalue) (- (.z _returnvalue) 3e+02)) (Transformation|GetWorldRotation _petite_porte_mobile) false false (Variables|/Game/Blueprints/BP_Door/BP_Door.BP_Door_C|GetOpeningDoorTime _bp_doortoopen) false))))))

(event EventBeginPlay
  (for _array_element (Variables|Default|GetBP_SteleToActivate)
    (Variables|/Game/Blueprints/BP_Steles/BP_StelesMother.BP_StelesMother_C|SetIsActivateByLevelButton _array_element false)))

(event Collision|EventActorBeginOverlap
  (params (OtherActor :type Actor%20Object%20Reference)))

(event EventTick
  (params (DeltaSeconds :type Float%20%28single-precision%29)))

(fn ConstructionScript
  ;[1 1 1] Set la variable de texte à afficher au départ
  (Rendering|Components|TextRender|SetText (Variables|Default|GetTXT_ButtonOnGround) (Variables|Default|GetTextToDisplay)))