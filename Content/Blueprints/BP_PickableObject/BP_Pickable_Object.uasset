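; Pickable object actor that hovers up and down and shows a collect prompt to nearby players.
; Tick bobs it with swept local Z offsets, reversing at bounds of an accumulator randomly seeded on BeginPlay; movement per frame is not delta-scaled.
; On the server, capsule overlaps have BP_PlayerProto add or remove the W_ClickToCollect widget through its client functions.
; The collection itself is not handled here.
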(event OnComponentBeginOverlap(Capsule)
  (params (OverlappedComponent :type Primitive%20Component%20Object%20Reference) (OtherActor :type Actor%20Object%20Reference) (OtherComp :type Primitive%20Component%20Object%20Reference) (OtherBodyIndex :type Integer) (bFromSweep :type Boolean) (SweepResult :type Hit%20Result%20Structure%20%28by%20ref%29))
  (Networking|SwitchHasAuthority
    (:Authority
      (bind _asbp_player_proto (Utilities|Casting|CastToBP_PlayerProto OtherActor))
      (Default|ClientAddWidgetbyClass _asbp_player_proto "/Game/Blueprints/BP_PickableObject/W_ClickToCollect.W_ClickToCollect_C"))))

(event OnComponentEndOverlap(Capsule)
  (params (OverlappedComponent :type Primitive%20Component%20Object%20Reference) (OtherActor :type Actor%20Object%20Reference) (OtherComp :type Primitive%20Component%20Object%20Reference) (OtherBodyIndex :type Integer))
  (Networking|SwitchHasAuthority
    (:Authority
      (bind _asbp_player_proto (Utilities|Casting|CastToBP_PlayerProto OtherActor))
      (Default|ClientRemoveAllWidgetbyClass _asbp_player_proto "/Game/Blueprints/BP_PickableObject/W_ClickToCollect.W_ClickToCollect_C"))))

(event EventBeginPlay
  (Variables|Default|SetLevitateValue (Math|Random|RandomFloatinRange 0.0 (Variables|Default|GetMaxLevitateValue))))

(event EventTick
  (params (DeltaSeconds :type Float%20%28single-precision%29))
  (Variables|Default|SetLevitateValue (+ (* DeltaSeconds (Variables|Default|GetLevitateFactor)) (Variables|Default|GetLevitateValue)))
  (Utilities|FlowControl|Sequence
    (:then_0
      (if (or (and (> (Variables|Default|GetLevitateValue) (Variables|Default|GetMaxLevitateValue)) (Variables|Default|GetObjectGoUp)) (and (< (Variables|Default|GetLevitateValue) 0.0) (not (Variables|Default|GetObjectGoUp))))
        (Variables|Default|SetLevitateFactor (- 0.0 (Variables|Default|GetLevitateFactor)))
        (Variables|Default|SetObjectGoUp (not (Variables|Default|GetObjectGoUp)))))
    (:then_1
      (Transformation|AddActorLocalOffset (Math|Vector|MakeVector 0.0 0.0 (Variables|Default|GetLevitateFactor)) true false))))

(fn ConstructionScript)