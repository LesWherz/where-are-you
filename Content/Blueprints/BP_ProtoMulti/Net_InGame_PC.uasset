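; Net_InGame_PC is an in-game player controller, apparently for a multiplayer prototype, that toggles a pause menu from the Escape_Pause input action.
; A FlipFlop alternates between creating and showing a Net_PauseMenu_W widget with a visible cursor and Game-and-UI input, and removing it to restore game-only input.
; The menu is built fresh on each opening, and the game itself is not paused here.
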(event Input|ActionEvents|InputActionEscape_Pause
  (params (Key :type Key%20Structure))
  (:Pressed
    (Utilities|FlowControl|FlipFlop
      (:A
        (bind _returnvalue (UserInterface|CreateWidget "/Game/Blueprints/BP_ProtoMulti/Net_Widget/Net_Multiplayer/Net_PauseMenu_W.Net_PauseMenu_W_C" (Game|GetPlayerController 0)))
        (UserInterface|Viewport|AddtoViewport _returnvalue 0)
        (Variables|Default|SetbShowMouseCursor true)
        (Input|SetInputModeGameandUI (Game|GetPlayerController 0) _returnvalue "DoNotLock" false))
      (:B
        (Variables|Default|SetbShowMouseCursor false)
        (Widget|RemovefromParent _returnvalue)
        (Input|SetInputModeGameOnly self)))))

(fn ConstructionScript)