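; Player controller for the networked main menu, which puts up the menu widgets and handles intro skipping and ready toggles.
; On BeginPlay, when enabled, it shows the lobby widget in the listen-server opening level, otherwise the normal menu with intro.
; Space or gamepad bottom button fades the intro out to the menu once.
; ToggleReady sets host or client readiness on GS_Menu, then triggers its launch-timer check; LoadMenu opens a level and creates Net_MainMenu_W.
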(event Custom|ToggleReady
  (params (IsServer :type Boolean) (Checked :type Boolean))
  (bind _as_gs_menu (Variables|Default|GetAs%20GS%20Menu))
  (if IsServer
    (Variables|/Game/Blueprints/GS_Menu.GS_Menu_C|SethostReady _as_gs_menu Checked)
    (else
      (Variables|/Game/Blueprints/GS_Menu.GS_Menu_C|SetclientReady _as_gs_menu Checked)))
  (Default|CheckifLaunchTimer _as_gs_menu))

(event EventBeginPlay
  (bind _asgs_menu (Utilities|Casting|CastToGS_Menu (Game|GetGameState)))
  (Variables|Default|SetAs%20GS%20Menu _asgs_menu)
  (if (Variables|Default|GetSHOW-NEW-MENU)
    (bind _returnvalue (Game|GetCurrentLevelName true))
    (if (Utilities|Enum|Equal(Enum) _returnvalue "L_GameOpening_listen")
      (bind _returnvalue_2 (UserInterface|CreateWidget "/Game/Assets/UI/Widgets/W_NewMenu_Lobby.W_NewMenu_Lobby_C"))
      (Utilities|IsValid _returnvalue_2
        (:Is%20Valid
          (UserInterface|Viewport|AddtoViewport _returnvalue_2 0)))
      (else
        (bind _returnvalue_3 (UserInterface|CreateWidget "/Game/Assets/UI/Widgets/W_NewMenu.W_NewMenu_C"))
        (Utilities|FlowControl|Sequence
          (:then_0
            (Variables|Default|SetNormalMenu true)
            (bind _output_get (Variables|Default|SetW%20New%20Menu _returnvalue_3))
            (Utilities|IsValid _output_get
              (:Is%20Valid
                (UserInterface|Viewport|AddtoViewport _output_get 0))))
          (:then_1
            (if (Variables|Default|GetNormalMenu)
              (Variables|Default|SetNewMenuIntro (Variables|Default|GetW%20New%20Menu)))))))))

(event Input|GamepadEvents|GamepadFaceButtonBottom
  (params (Key :type Key%20Structure :default "None"))
  (bind _newmenuintro (Variables|Default|GetNewMenuIntro))
  (:Pressed
    (if (not (Variables|Default|GetIntroAnimDone))
      (Class|UserWidget|StopAnimation _newmenuintro (Variables|/Game/Assets/UI/Widgets/W_NewMenu.W_NewMenu_C|GetIntro_Wait _newmenuintro))
      (UserInterface|Animation|PlayAnimation _newmenuintro (Variables|/Game/Assets/UI/Widgets/W_NewMenu.W_NewMenu_C|GetIntro_FadeOut_ToMenu _newmenuintro) 0.0 1 "Forward" 1.0 false)
      (Variables|Default|SetIntroAnimDone true))))

(event Input|KeyboardEvents|SpaceBar
  (params (Key :type Key%20Structure :default "None"))
  (bind _newmenuintro (Variables|Default|GetNewMenuIntro))
  (:Pressed
    (if (not (Variables|Default|GetIntroAnimDone))
      (Class|UserWidget|StopAnimation _newmenuintro (Variables|/Game/Assets/UI/Widgets/W_NewMenu.W_NewMenu_C|GetIntro_Wait _newmenuintro))
      (UserInterface|Animation|PlayAnimation _newmenuintro (Variables|/Game/Assets/UI/Widgets/W_NewMenu.W_NewMenu_C|GetIntro_FadeOut_ToMenu _newmenuintro) 0.0 1 "Forward" 1.0 false)
      (Variables|Default|SetIntroAnimDone true))))

(fn ConstructionScript)

(fn LoadMenu
  (params (Level :type World%20Soft%20Object%20Reference))
  (Game|OpenLevel(byObjectReference) Level)
  (bind _returnvalue (UserInterface|CreateWidget "/Game/Blueprints/BP_ProtoMulti/Net_Widget/Net_Multiplayer/Net_MainMenu_W.Net_MainMenu_W_C" self))
  (UserInterface|Viewport|AddtoViewport _returnvalue 0)
  (return))