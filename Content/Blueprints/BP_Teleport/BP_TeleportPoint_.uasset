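; Teleport trigger actor that moves the player to the location of a linked TeleportPointLocation actor.
; On box overlap with BP_PlayerProto, it disables input and shows a W_WaitingToTeleport widget for a short fixed delay.
; It then sets the player to the world location of the target's SMCubeLocation component, removes the widget and restores input.
; The construction script applies LightIntensity to its point light.
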(event OnComponentBeginOverlap(Box)
  (params (OverlappedComponent :type Primitive%20Component%20Object%20Reference) (OtherActor :type Actor%20Object%20Reference) (OtherComp :type Primitive%20Component%20Object%20Reference) (OtherBodyIndex :type Integer) (bFromSweep :type Boolean) (SweepResult :type Hit%20Result%20Structure%20%28by%20ref%29))
  (bind _returnvalue (Game|GetPlayerController 0))
  (bind _asbp_player_proto (Utilities|Casting|CastToBP_PlayerProto OtherActor))
  (Input|DisableInput _asbp_player_proto _returnvalue)
  (bind _returnvalue_2 (UserInterface|CreateWidget "/Game/Assets/UI/Widgets/W_WaitingToTeleport.W_WaitingToTeleport_C"))
  (UserInterface|Viewport|AddtoViewport _returnvalue_2 0)
  (Utilities|FlowControl|Delay 3.0)
  (Transformation|SetActorLocation _asbp_player_proto (Transformation|GetWorldLocation (Variables|/Game/Blueprints/BP_Teleport/BP_TeleportPointLocation.BP_TeleportPointLocation_C|GetSM_CubeLocation (Variables|Default|GetTeleportPointLocation))) false false)
  (Widget|RemovefromParent _returnvalue_2)
  (Input|EnableInput _asbp_player_proto _returnvalue))

(event EventBeginPlay)

(event Collision|EventActorBeginOverlap
  (params (OtherActor :type Actor%20Object%20Reference)))

(event EventTick
  (params (DeltaSeconds :type Float%20%28single-precision%29)))

(fn ConstructionScript
  (Rendering|Components|Light|SetIntensity (Variables|Default|GetPointLight) (Variables|Default|GetLightIntensity)))