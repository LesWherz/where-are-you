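; Two-player airlock (sas) between level sections that hides level streaming behind a pair of sliding doors.
; Door A opens on overlap, then closes through player controller calls once two players are counted inside.
; Closing swaps the streamed levels, while Tick polls loading into separate server and client flags.
; When both flags are set, it resets players and opens door B; countdown/teleport logic is disconnected.
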(event OnComponentBeginOverlap(BoxDetectA)
  (params (OverlappedComponent :type Primitive%20Component%20Object%20Reference) (OtherActor :type Actor%20Object%20Reference) (OtherComp :type Primitive%20Component%20Object%20Reference) (OtherBodyIndex :type Integer) (bFromSweep :type Boolean) (SweepResult :type Hit%20Result%20Structure%20%28by%20ref%29))
  ;[0.126 1 0.07761] OPEN THE DOOR A
  (if (Variables|Default|GetcanOpen)
    (Variables|Default|SetcanOpen false)
    (CallFunction|OpenPorteA)))

(event OnComponentBeginOverlap(DetectPeopleInside)
  (params (OverlappedComponent :type Primitive%20Component%20Object%20Reference) (OtherActor :type Actor%20Object%20Reference) (OtherComp :type Primitive%20Component%20Object%20Reference) (OtherBodyIndex :type Integer) (bFromSweep :type Boolean) (SweepResult :type Hit%20Result%20Structure%20%28by%20ref%29))
  (bind _playercontrollerref (Variables|Default|GetPlayerControllerREF))
  ;[0.1906 0.2156 1] INCREMENT NUMBER OF PEOPLE INSIDE
  (if (not (Variables|Default|GetisClosed))
    (bind _asbp_player_proto (Utilities|Casting|CastToBP_PlayerProto (Pawn|GetControlledPawn (Game|GetPlayerController 0))))
    (if (== OtherComp (Variables|/Script/Engine.Character|GetCapsuleComponent _asbp_player_proto))
      (Utilities|IsValid _playercontrollerref
        (:Is%20Valid
          (Default|CLIENTIncrementNbrOfPlayerSAS _playercontrollerref self))))))

(event OnComponentEndOverlap(DetectPeopleInside)
  (params (OverlappedComponent :type Primitive%20Component%20Object%20Reference) (OtherActor :type Actor%20Object%20Reference) (OtherComp :type Primitive%20Component%20Object%20Reference) (OtherBodyIndex :type Integer))
  ;[1 1 1] DECREMENT NUMBER OF PEOPLE INSIDE
  (bind _asbp_player_proto (Utilities|Casting|CastToBP_PlayerProto (Pawn|GetControlledPawn (Game|GetPlayerController 0))))
  (if (== OtherComp (Variables|/Script/Engine.Character|GetCapsuleComponent _asbp_player_proto))
    (Math|Integer|DecrementInt (Variables|Default|GetNumberOfPeopleInside))))

(event Custom|Load%20Needed%20LEVELS
  ;[1 1 1] RESET PLAYERS
  (for _array_element (Variables|Default|GetLevelToUnload)
    (Class|GameplayStatics|UnloadStreamLevelbySoftObjectPtr _array_element false))
  (for _array_element_2 (Variables|Default|GetLevelToLoad)
    (Game|LoadStreamLevel(byName) _array_element_2 true)))

(event Custom|IncrementNumberOfPlayerInside
  ;[0.1906 0.2156 1] INCREMENT NUMBER OF PEOPLE INSIDE
  (bind _result (Math|Integer|IncrementInt (Variables|Default|GetNumberOfPeopleInside))
    (:%20%20
      (if (>= _result 2)
        (Variables|Default|SetisClosed true)
        (Default|CLIENTCloseDoorA (Variables|Default|GetPlayerControllerREF) self)))))

(event Custom|CloseDoorA
  (bind _porte_a (Variables|Default|GetPorte_A))
  (bind _relativelocation (Variables|/Script/Engine.SceneComponent|GetRelativeLocation _porte_a))
  ;[1 0 0.07821] CLOSE DOOR A
  (Collision|SetCollisionEnabled (Variables|Default|GetSecurityFromRunningOut) "QueryAndPhysics")
  (Components|MoveComponentTo _porte_a (Math|Vector|MakeVector (.x _relativelocation) (.y _relativelocation) (+ (.z _relativelocation) -3e+02)) "0, 0, 0" false false 2.0 false)
  (CallFunction|LoadNeededLEVELS))

(event Custom|DecrementNbrPlayerInside
  ;[1 1 1] DECREMENT NUMBER OF PEOPLE INSIDE
  (Math|Integer|DecrementInt (Variables|Default|GetNumberOfPeopleInside)))

(event Custom|OpenPorteA
  (bind _porte_a (Variables|Default|GetPorte_A))
  (bind _relativelocation (Variables|/Script/Engine.SceneComponent|GetRelativeLocation _porte_a))
  ;[0.126 1 0.07761] OPEN THE DOOR A
  (Components|MoveComponentTo _porte_a (Math|Vector|MakeVector (.x _relativelocation) (.y _relativelocation) (+ (.z _relativelocation) 3e+02)) "0, 0, 0" false false 2.0 false)
  (CallFunction|PlaySoundOpeningDoor))

(event Custom|OpenDoorB
  (bind _porte_b (Variables|Default|GetPorte_B))
  (bind _relativelocation (Variables|/Script/Engine.SceneComponent|GetRelativeLocation _porte_b))
  ;[1 1 1] RESET PLAYERS
  (Variables|Default|SetDoorBOpenned true)
  (Utilities|IsValid (Variables|Default|GetPlayerControllerREF)
    (:Is%20Valid
      (Rendering|Components|Light|SetLightColor (Variables|Default|GetPointLight) (Math|Color|MakeColor 0.0 255.0 255.0) true)
      (Components|MoveComponentTo _porte_b (Math|Vector|MakeVector (.x _relativelocation) (.y _relativelocation) (+ (.z _relativelocation) 3e+02)) "0, 0, 0" false false 2.0 false))))

(event Custom|Reset%20Players
  ;[1 1 1] RESET PLAYERS
  (bind _outactors (Actor|GetAllActorsOfClass "/Game/Assets/Character/Blueprint/PC_PlayerProto.PC_PlayerProto_C"))
  (for _array_element _outactors
    (Networking|SwitchHasAuthority
      (:Authority
        (Default|SERVERResetPlayer _array_element self))
      (:Remote
        (Default|CLIENTResetPlayer _array_element self)))
    (CallFunction|OpenDoorB)))

(event EventBeginPlay
  (Collision|SetCollisionEnabled (Variables|Default|GetSecurityFromRunningOut) "NoCollision")
  (bind _aspc_player_proto (Utilities|Casting|CastToPC_PlayerProto (Game|GetPlayerController 0)))
  (Variables|Default|SetPlayerControllerREF _aspc_player_proto)
  (if (Variables|Default|GetSpawningSAS)
    _
    (else
      (Variables|/Script/Engine.PrimitiveComponent|SetbGenerateOverlapEvents (Variables|Default|GetDetectPeopleInside) true)))
  (Variables|Default|SetisInit true))

(event Custom|PlaySoundOpeningDoor)

(event Custom|PlaySoundScanPlayer)

(event Custom|DecompteBeforeTP
  ;[1 1 1] REMPLACER LES PRINTS PAR DES SONS
)

(event Custom|TeleportToNextLevel)

(event Custom|AreAllLevelsLoaded
  ;[0.07549 1 0.2686] DETECTE SI LE JOUEUR A CHARGE TOUTE LES SCENES
  (bind _array_element (Utilities|Array|ForEachLoopwithBreak (Variables|Default|GetLevelToLoad))
    (:LoopBody
      (Utilities|IsValid (Class|GameplayStatics|GetStreamingLevel _array_element)
        (:Is%20Valid
          (if (Class|LevelStreaming|IsLevelLoaded (Class|GameplayStatics|GetStreamingLevel _array_element))
            (Math|Integer|IncrementInt (Variables|Default|GetNbrOfLoadedScene))))))
    (:Completed
      (if (== (Utilities|Array|Length (Variables|Default|GetLevelToLoad)) (Variables|Default|GetNbrOfLoadedScene))
        (Networking|SwitchHasAuthority
          (:Authority
            (Variables|Default|SetServerPCHasAllLoaded true))
          (:Remote
            (Variables|Default|SetClientPCHasAllLoaded true)))
        (else
          (Variables|Default|SetNbrOfLoadedScene 0))))))

(event EventTick
  (params (DeltaSeconds :type Float%20%28single-precision%29))
  ;[0.8292 1 0.0585] OUVRE LA PORTE SI TOUT LES JOUEURS ON CHARGE LES NIVEAUX
  (if (and (Variables|Default|GetServerPCHasAllLoaded) (Variables|Default|GetClientPCHasAllLoaded))
    (if (not (Variables|Default|GetDoorBOpenned))
      (CallFunction|ResetPlayers))
    (elif (Variables|Default|GetisInit)
      (CallFunction|AreAllLevelsLoaded))))

(fn ConstructionScript)

(fn OnTaskEnd
  (bind _result (Math|Integer|DecrementInt (Variables|Default|GetCountAsync))
    (:%20%20
      (if (<= _result 0)
        (Development|PrintString "TOUT CHARGE")
        (else
          (Development|PrintString "PAS FINI"))))))