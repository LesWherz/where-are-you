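; GS_Menu is a menu game state, going by its name, that launches the selected level once both host and client are ready.
; CheckIfLaunchTimer plays a timeline that feeds a visible countdown value, stopping and zeroing it if either side becomes unready.
; When the timeline finishes, it shows a "Starting Game" message widget, then runs a servertravel console command to the selected level after a brief delay.
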(event Custom|CheckIfLaunchTimer
  (if (and (Variables|Default|GetclientReady) (Variables|Default|GethostReady))
    (Variables|Default|SetVisibleTimer true)
    (bind _newtrack_0 (Timeline|Timeline_0 PlayFromStart)
      (:Update
        (if (and (Variables|Default|GetclientReady) (Variables|Default|GethostReady))
          (Variables|Default|SetVisibleTimerValue _newtrack_0)
          (else
            (Variables|Default|SetVisibleTimerValue 0.0)
            (Variables|Default|SetVisibleTimer false)
            (Timeline|Timeline_0 Stop))))
      (:Finished
        (CallFunction|AddLaunchMessage)
        (Utilities|FlowControl|Delay 0.02)
        (CallFunction|LaunchMap)))
    (else
      (Variables|Default|SetVisibleTimerValue 0.0)
      (Timeline|Timeline_0 Stop))))

(event Custom|LaunchMap
  (Development|ExecuteConsoleCommand (Utilities|String|Append "servertravel " (Variables|Default|GetSelectedLevel)) 0))

(event Custom|AddLaunchMessage
  (bind _returnvalue (UserInterface|CreateWidget "/Game/Assets/UI/Widgets/W_ErrorMsg.W_ErrorMsg_C" 0 "Starting Game" (Utilities|String|Append "Opening " (Variables|Default|GetSelectedLevel))))
  (UserInterface|Viewport|AddtoViewport _returnvalue 0))

(event EventBeginPlay)

(fn ConstructionScript)

(fn OnRepHostReady)