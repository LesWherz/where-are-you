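; BP_Door is a puzzle door that slides its mobile panel upward by a set height over a set time.
; Three events open it: a digicode counter matching the scene's digicode total, a key, or a stele whose gameplay tag matches the door's.
; Key and stele openings set an IsOpen flag to run only once, while the digicode path skips that check and no event closes the door.
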(event Custom|OpenDoorDIGICODE
  (params (MoreOrLess :type Integer))
  (bind _petite_porte_mobile (Variables|Default|GetPetite_Porte_Mobile))
  (bind _relativelocation (Variables|/Script/Engine.SceneComponent|GetRelativeLocation _petite_porte_mobile))
  ;[1 0.03684 0.608] OPEN DOOR WITH DIGICODE
  (bind _output_get (Variables|Default|SetnumberOfCorrectDigicode (+ (Variables|Default|GetnumberOfCorrectDigicode) MoreOrLess)))
  (Development|PrintString (Utilities|String|ToString(Integer) _output_get))
  (if (== _output_get (Variables|Default|GetnumberOfDigicodeInScene))
    (Components|MoveComponentTo (Variables|Default|GetPetite_Porte_Mobile) (Math|Vector|MakeVector (.x _relativelocation) (.y _relativelocation) (+ (.z _relativelocation) (Variables|Default|GetOpenningHeight))) (Variables|/Script/Engine.SceneComponent|GetRelativeRotation _petite_porte_mobile) false false (Variables|Default|GetOpeningDoorTime) false)))

(event Custom|OpenDoorSTELE
  (params (GameplayTAG :type Gameplay%20Tag%20Structure))
  (bind _petite_porte_mobile (Variables|Default|GetPetite_Porte_Mobile))
  (bind _relativelocation (Variables|/Script/Engine.SceneComponent|GetRelativeLocation _petite_porte_mobile))
  ;[0.1249 1 0.7683] OPEN DOOR WITH STELE
  (if (== GameplayTAG (Variables|Default|GetGameplayTagDoorStele))
    (if (not (Variables|Default|GetisOpen))
      (Development|PrintString "DOOR OPENING")
      (Variables|Default|SetisOpen true)
      (Components|MoveComponentTo (Variables|Default|GetPetite_Porte_Mobile) (Math|Vector|MakeVector (.x _relativelocation) (.y _relativelocation) (+ (.z _relativelocation) (Variables|Default|GetOpenningHeight))) (Variables|/Script/Engine.SceneComponent|GetRelativeRotation _petite_porte_mobile) false false (Variables|Default|GetOpeningDoorTime) false))))

(event Custom|OpenDoorKey
  (bind _petite_porte_mobile (Variables|Default|GetPetite_Porte_Mobile))
  (bind _relativelocation (Variables|/Script/Engine.SceneComponent|GetRelativeLocation _petite_porte_mobile))
  ;[0.9683 1 0] OPEN DOOR WITH THE A KEY
  (if (not (Variables|Default|GetisOpen))
    (Variables|Default|SetisOpen true)
    (Components|MoveComponentTo (Variables|Default|GetPetite_Porte_Mobile) (Math|Vector|MakeVector (.x _relativelocation) (.y _relativelocation) (+ (.z _relativelocation) (Variables|Default|GetOpenningHeight))) (Variables|/Script/Engine.SceneComponent|GetRelativeRotation _petite_porte_mobile) false false (Variables|Default|GetOpeningDoorTime) false)))

(fn ConstructionScript)