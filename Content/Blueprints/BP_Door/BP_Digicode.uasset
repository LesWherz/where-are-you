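; Digicode keypad that opens its linked door when the correct code is entered.
; Each button press plays a beep and feeds Newstring, which appends up to three characters to the screen text, clears it on X or checks it against CorrectCode on V.
; A correct code opens the door, then after a five-second delay clears the keypad and sends the reverse call to the door.
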(event Custom|CodeIsCorrect
  (bind _door (Variables|Default|GetDoor))
  (Variables|Default|SetisCorrect true)
  (Default|OpenDoorDIGICODE _door 1)
  (Utilities|FlowControl|Delay 5.0)
  (Development|PrintString "RESET DIGICODE")
  (CallFunction|ResetDigicode)
  (Default|OpenDoorDIGICODE _door -1)
  (Variables|Default|SetisCorrect false))

(event Custom|OnButtonPressed
  (params (NumberValue :type String))
  (CallFunction|Newstring NumberValue)
  (Rendering|Components|TextRender|SetText (Variables|Default|GetNumbersInScreen) (Variables|Default|GetValueScreen))
  (Audio|PlaySoundatLocation "/Game/Sounds/Beeps/Beep_Code.Beep_Code" (Transformation|GetWorldLocation (Variables|Default|GetCube)) "0, 0, 0" 1.0 1.0 0.0 0 0 0))

(event Custom|ResetDigicode
  (Variables|Default|SetnumberOfCharacter 0)
  (bind _output_get (Variables|Default|SetValueScreen (Utilities|Text|ToText(String) "")))
  (Rendering|Components|TextRender|SetText (Variables|Default|GetNumbersInScreen) _output_get))

(fn ConstructionScript)

(fn Newstring
  (params (B :type String))
  (switch string B
    (:Default
      ;[0 1 0.1179] SI NOMBRE AJOUTE
      (if (< (Variables|Default|GetnumberOfCharacter) 3)
        (Math|Integer|IncrementInt (Variables|Default|GetnumberOfCharacter)
          (:%20%20
            (Variables|Default|SetValueScreen (Utilities|Text|ToText(String) (Utilities|String|Append (Utilities|String|ToString(Text) (Variables|/Script/Engine.TextRenderComponent|GetText (Variables|Default|GetNumbersInScreen))) B)))
            (return)))))
    (:x
      ;[1 0.04504 0] DELETE ALL
      (Variables|Default|SetnumberOfCharacter 0)
      (Variables|Default|SetValueScreen (Utilities|Text|ToText(String) ""))
      (return))
    (:v
      ;[1 0.8681 0.09452] VERIF CODE
      (if (not (Variables|Default|GetisCorrect))
        (if (Utilities|Enum|Equal(Enum) (Variables|Default|GetCorrectCode) (Variables|Default|GetValueScreen))
          (Development|PrintString "CODE CORRECT")
          (CallFunction|CodeIsCorrect)
          (else
            (Development|PrintString "CODE FAUX")))))))

(fn OnRepValueScreen)