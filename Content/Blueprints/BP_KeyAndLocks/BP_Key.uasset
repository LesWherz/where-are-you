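; BP_Key is a key actor that players can pick up, drop and use on interactable objects, passing itself to the object's OnBeginInteract.
; Pickup disables the Box's physics and collision, and a drop re-enables them unless it comes from an interaction.
; It tracks its holder so DropMe can request a drop through that player's AC_PickUp via DropServer.
; Empty key events serve as hooks for custom logic.
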(event EventOnInteracted
  (params (interactableObject :type I%20Interactable%20Object%20Interface%20%28by%20ref%29))
  (|CallParentFunction interactableObject)
  (Class|IInteractableObject|OnBeginInteract interactableObject self)
  (CallFunction|OnKeyInteractedwithElement))

(event EventDropMe
  (bind _playerhowpickmeup (Variables|Default|GetPlayerHowPickMeUp))
  (Utilities|IsValid _playerhowpickmeup
    (:Is%20Valid
      (Default|DropServer (Actor|GetComponentbyClass _playerhowpickmeup "/Game/Assets/Character/Blueprint/AC_PickUp.AC_PickUp_C") false))))

(event EventOnDropped
  (params (playerHowDrop :type Actor%20Object%20Reference) (fromInteraction :type Boolean))
  (|CallParentFunction playerHowDrop fromInteraction)
  (Variables|Default|SetPlayerHowPickMeUp 0)
  (if fromInteraction
    (CallFunction|DisablePhysics)
    (CallFunction|OnKeyDropped)
    (else
      (CallFunction|EnablePhysics)
      (CallFunction|OnKeyDropped))))

(event EventOnPickedUp
  (params (playerHowPickup :type Actor%20Object%20Reference))
  (|CallParentFunction playerHowPickup)
  (Variables|Default|SetPlayerHowPickMeUp playerHowPickup)
  (CallFunction|DisablePhysics)
  (CallFunction|OnKeyPickedUp))

(event Custom|OnKeyDropped
  ;[1 1 1] Events - Rajouter la logique des évènements qui se produisent quand on veut
)

(event Custom|OnKeyInteractedWithElement
  ;[1 1 1] Events - Rajouter la logique des évènements qui se produisent quand on veut
)

(event Custom|OnKeyPickedUp
  ;[1 1 1] Events - Rajouter la logique des évènements qui se produisent quand on veut
)

(fn ConstructionScript)

(fn PlayAnimation)

(fn DisablePhysics
  (bind _box (Variables|Default|GetBox))
  (Physics|SetSimulatePhysics _box false)
  (Physics|SetEnableGravity _box false)
  (Collision|SetCollisionEnabled _box "NoCollision"))

(fn EnablePhysics
  (bind _box (Variables|Default|GetBox))
  (Physics|SetSimulatePhysics _box true)
  (Physics|SetEnableGravity _box true)
  (Collision|SetCollisionEnabled _box "QueryAndPhysics"))