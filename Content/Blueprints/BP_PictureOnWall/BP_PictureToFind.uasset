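; BP_PictureToFind is one corner piece of a wall-picture alignment puzzle, showing a decal for its side.
; A manager instance gathers all pieces and reveals their text while StartDetection, set by box overlap, is active.
; IsInFront projects corners to screen, printing whether all are visible.
; Success blends to a camera and lights outer borders, but the diagonal/angle validation and hold timer that would trigger it are disconnected.
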(event OnActorBeginOverlap(BoxStartDetection)
  (params (OverlappedActor :type Actor%20Object%20Reference) (OtherActor :type Actor%20Object%20Reference))
  ;[1 1 1] START DETECTION SI ON EST DANS LA BOX
  (Variables|Default|SetStartDetection true))

(event OnActorEndOverlap(BoxStartDetection)
  (params (OverlappedActor :type Actor%20Object%20Reference) (OtherActor :type Actor%20Object%20Reference))
  ;[1 1 1] START DETECTION SI ON EST DANS LA BOX
  (Variables|Default|SetStartDetection false))

(event Custom|IsInFront
  (Networking|SwitchHasAuthority
    (:Authority
      (bind (_upleft _upright _downright _downleft _allinscreen_) (CallFunction|GetScreenLocation))
      (Development|PrintString (Utilities|String|ToString(Boolean) _allinscreen_)))))

(event Custom|Success
  (bind _returnvalue (Game|GetPlayerController 0))
  (bind _returnvalue_2 (Game|GetPlayerController 0))
  (Variables|Default|SetNotFounded false)
  (Game|Player|SetViewTargetwithBlend _returnvalue_2 (Variables|Default|GetCamera) 1.0 "VTBlend_Linear" 0.0 false)
  (Input|SetIgnoreMoveInput _returnvalue_2 true)
  (Utilities|FlowControl|Delay 1.0)
  (CallFunction|TurnonEverything)
  (Utilities|FlowControl|Delay 0.5)
  (Game|Player|SetViewTargetwithBlend _returnvalue (Game|GetPlayerCharacter 0) 0.1 "VTBlend_Linear" 0.0 false)
  (Input|SetIgnoreMoveInput _returnvalue false))

(event EventBeginPlay
  ;[1 1 1] Turn Off all the border lights and reset the reference to all the other pictures
  (Development|SetHiddeninGame (Variables|Default|GetTop) true false)
  (Development|SetHiddeninGame (Variables|Default|GetDown) true false)
  (Development|SetHiddeninGame (Variables|Default|GetLeft) true false)
  (Development|SetHiddeninGame (Variables|Default|GetRight) true false)
  (if (Variables|Default|GetIsManager)
    (CallFunction|SaveAllRefOfOthersPicture)
    (CallFunction|SetVisualDecal (Variables|Default|GetEnumSideOfPicture))
    (elif (not (Variables|Default|GetIsCopy))
      (CallFunction|SetVisualDecal (Variables|Default|GetEnumSideOfPicture)))))

(event EventTick
  (params (DeltaSeconds :type Float%20%28single-precision%29))
  (if (Math|Boolean|ANDBoolean (Variables|Default|GetStartDetection) (Variables|Default|GetIsManager) (Variables|Default|GetNotFounded))
    (for _array_element (Variables|Default|GetOtherPictures)
      (Development|SetHiddeninGame (Variables|BP_PictureToFind_C|GetTextRender _array_element) false false))))

(fn ConstructionScript)

(fn GetScreenLocation
  (bind _returnvalue (Viewport|GetViewportSize))
  (for _array_element (Variables|Default|GetOtherPictures)
    (switch Utilities|FlowControl|Switch|SwitchonESideOfPicture (Variables|BP_PictureToFind_C|GetEnumSideOfPicture _array_element)
      (:NewEnumerator0
        (LocalVariables|SetUpLeftLocal (.ScreenPosition (Class|GameplayStatics|ProjectWorldtoScreen (Game|GetPlayerController 0) (Transformation|GetWorldLocation (Variables|BP_PictureToFind_C|GetExtremityForCalcul _array_element)) false))))
      (:NewEnumerator1
        (LocalVariables|SetUpRightLocal (.ScreenPosition (Class|GameplayStatics|ProjectWorldtoScreen (Game|GetPlayerController 0) (Transformation|GetWorldLocation (Variables|BP_PictureToFind_C|GetExtremityForCalcul _array_element)) false))))
      (:NewEnumerator2
        (LocalVariables|SetDownLeftLocal (.ScreenPosition (Class|GameplayStatics|ProjectWorldtoScreen (Game|GetPlayerController 0) (Transformation|GetWorldLocation (Variables|BP_PictureToFind_C|GetExtremityForCalcul _array_element)) false))))
      (:NewEnumerator3
        (LocalVariables|SetDownRightLocal (.ScreenPosition (Class|GameplayStatics|ProjectWorldtoScreen (Game|GetPlayerController 0) (Transformation|GetWorldLocation (Variables|BP_PictureToFind_C|GetExtremityForCalcul _array_element)) false))))))
  (return (LocalVariables|GetUpLeftLocal) (LocalVariables|GetUpRightLocal) (LocalVariables|GetDownLeftLocal) (LocalVariables|GetDownRightLocal) (Math|Boolean|ANDBoolean (Math|Boolean|ANDBoolean (< (.x (LocalVariables|GetUpLeftLocal)) (.x _returnvalue)) (> (.x (LocalVariables|GetUpLeftLocal)) 0.0) (< (.y (LocalVariables|GetUpLeftLocal)) (.y _returnvalue)) (> (.y (LocalVariables|GetUpLeftLocal)) 0.0)) (Math|Boolean|ANDBoolean (< (.x (LocalVariables|GetUpRightLocal)) (.x _returnvalue)) (> (.x (LocalVariables|GetUpRightLocal)) 0.0) (< (.y (LocalVariables|GetUpRightLocal)) (.y _returnvalue)) (> (.y (LocalVariables|GetUpRightLocal)) 0.0)) (Math|Boolean|ANDBoolean (< (.x (LocalVariables|GetDownRightLocal)) (.x _returnvalue)) (> (.x (LocalVariables|GetDownRightLocal)) 0.0) (< (.y (LocalVariables|GetDownRightLocal)) (.y _returnvalue)) (> (.y (LocalVariables|GetDownRightLocal)) 0.0)) (Math|Boolean|ANDBoolean (< (.x (LocalVariables|GetDownLeftLocal)) (.x _returnvalue)) (> (.x (LocalVariables|GetDownLeftLocal)) 0.0) (< (.y (LocalVariables|GetDownLeftLocal)) (.y _returnvalue)) (> (.y (LocalVariables|GetDownLeftLocal)) 0.0)))))

(fn CalculDistanceBetweenPoints
  (params (U :type Vector%202D%20Structure) (V :type Vector%202D%20Structure))
  (return (Math|Float|Sqrt (+ (Math|Float|Square (- (.x V) (.x U))) (Math|Float|Square (- (.y V) (.y U)))))))

(fn TurnonEverything
  (for _array_element (Variables|Default|GetOtherPictures)
    (switch Utilities|FlowControl|Switch|SwitchonESideOfPicture (Variables|BP_PictureToFind_C|GetEnumSideOfPicture _array_element)
      (:NewEnumerator0
        (Development|SetHiddeninGame (Variables|BP_PictureToFind_C|GetTop _array_element) false false)
        (Rendering|SetVisibility (Variables|BP_PictureToFind_C|GetTop _array_element) true false)
        (Development|SetHiddeninGame (Variables|BP_PictureToFind_C|GetLeft _array_element) false false)
        (Rendering|SetVisibility (Variables|BP_PictureToFind_C|GetLeft _array_element) true false))
      (:NewEnumerator1
        (Development|SetHiddeninGame (Variables|BP_PictureToFind_C|GetTop _array_element) false false)
        (Rendering|SetVisibility (Variables|BP_PictureToFind_C|GetTop _array_element) true false)
        (Development|SetHiddeninGame (Variables|BP_PictureToFind_C|GetRight _array_element) false false)
        (Rendering|SetVisibility (Variables|BP_PictureToFind_C|GetRight _array_element) true false))
      (:NewEnumerator2
        (Development|SetHiddeninGame (Variables|BP_PictureToFind_C|GetDown _array_element) false false)
        (Rendering|SetVisibility (Variables|BP_PictureToFind_C|GetDown _array_element) true false)
        (Development|SetHiddeninGame (Variables|BP_PictureToFind_C|GetLeft _array_element) false false)
        (Rendering|SetVisibility (Variables|BP_PictureToFind_C|GetLeft _array_element) true false))
      (:NewEnumerator3
        (Development|SetHiddeninGame (Variables|BP_PictureToFind_C|GetDown _array_element) false false)
        (Rendering|SetVisibility (Variables|BP_PictureToFind_C|GetDown _array_element) true false)
        (Development|SetHiddeninGame (Variables|BP_PictureToFind_C|GetRight _array_element) false false)
        (Rendering|SetVisibility (Variables|BP_PictureToFind_C|GetRight _array_element) true false)))))

(fn CalculAngle
  (params (A :type Vector%202D%20Structure) (B :type Vector%202D%20Structure) (C :type Vector%202D%20Structure))
  (bind _returnvalue (CallFunction|CalculDistanceBetweenPoints (Math|Vector2D|MakeVector2D (.x A) (.y A)) (Math|Vector2D|MakeVector2D (.x B) (.y B))))
  (bind _output_get (LocalVariables|SetAB _returnvalue))
  (bind _returnvalue_2 (CallFunction|CalculDistanceBetweenPoints (Math|Vector2D|MakeVector2D (.x A) (.y A)) (Math|Vector2D|MakeVector2D (.x C) (.y C))))
  (bind _output_get_2 (LocalVariables|SetAC _returnvalue_2))
  (bind _returnvalue_3 (CallFunction|CalculDistanceBetweenPoints (Math|Vector2D|MakeVector2D (.x B) (.y B)) (Math|Vector2D|MakeVector2D (.x C) (.y C))))
  (bind _output_get_3 (LocalVariables|SetBC _returnvalue_3))
  (return (Class|KismetMathLibrary|DegAcos (/ (- (+ (Math|Float|Square _output_get) (Math|Float|Square _output_get_2)) (Math|Float|Square _output_get_3)) (* _output_get 2.0 _output_get_2)))))

(fn SaveAllRefOfOthersPicture
  (bind _outactors (Actor|GetAllActorsOfClass "BP_PictureToFind_C"))
  (for _array_element _outactors
    (Utilities|Array|Add (Variables|Default|GetOtherPictures) _array_element)))

(fn SetVisualDecal
  (params (PictureSide :type ESideOfPicture%20Enum :default "NewEnumerator0"))
  (bind _output_get (Variables|Default|SetEnumSideOfPicture PictureSide))
  (switch Utilities|FlowControl|Switch|SwitchonESideOfPicture _output_get
    (:NewEnumerator0
      (Rendering|Components|Decal|SetDecalMaterial (Variables|Default|GetDecal) (Variables|Materials|GetMaterialUpLeft)))
    (:NewEnumerator1
      (Rendering|Components|Decal|SetDecalMaterial (Variables|Default|GetDecal) (Variables|Materials|GetMaterialUpRight)))
    (:NewEnumerator2
      (Rendering|Components|Decal|SetDecalMaterial (Variables|Default|GetDecal) (Variables|Materials|GetMaterialDownLeft)))
    (:NewEnumerator3
      (Rendering|Components|Decal|SetDecalMaterial (Variables|Default|GetDecal) (Variables|Materials|GetMaterialDownRight)))))

(fn SaveRefOfOnePicture
  (params (Side :type ESideOfPicture%20Enum :default "NewEnumerator0"))
  (if (Variables|Default|GetIsManager)
    (for (_array_element _array_index) (Variables|Default|GetOtherPictures)
      (if (Utilities|Enum|Equal(Enum) Side (Variables|BP_PictureToFind_C|GetEnumSideOfPicture _array_element))
        (Utilities|Array|SetArrayElem (Variables|Default|GetOtherPictures) _array_index self)))
    (else
      (bind _manager (CallFunction|GetPictureManager))
      (CallFunction|SaveRefOfOnePicture _manager Side))))

(fn GetPictureManager
  (bind _outactors (Actor|GetAllActorsOfClass "BP_PictureToFind_C"))
  (for _array_element _outactors
    (if (Variables|BP_PictureToFind_C|GetIsManager _array_element)
      (return _array_element)))
  (return 0))