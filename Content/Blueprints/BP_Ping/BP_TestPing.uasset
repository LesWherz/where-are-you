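; BP_TestPing is a world ping marker whose text shows the player's distance to it in whole meters.
; On BeginPlay it caches the BP_PlayerProto character.
; While the ping is visible, Tick rotates the text to face that character's first-person camera and updates the floored distance.
; SetPingVisible toggles both the visibility flag and the actor's hidden-in-game state.
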(event EventBeginPlay
  (bind _asbp_player_proto (Utilities|Casting|CastToBP_PlayerProto (Game|GetPlayerCharacter 0)))
  (Variables|Default|SetCachedCharacter _asbp_player_proto))

(event EventTick
  (params (DeltaSeconds :type Float%20%28single-precision%29))
  (bind _pingtext (Variables|Default|GetPingText))
  (bind _returnvalue (Transformation|GetWorldLocation _pingtext))
  (if (and (Utilities|IsValid (Variables|Default|GetCachedCharacter)) (Variables|Default|GetIsPingVisible))
    (Transformation|SetWorldRotation (Variables|Default|GetPingText) (Math|Rotator|FindLookatRotation _returnvalue (Transformation|GetWorldLocation (Variables|/Game/Assets/Character/Blueprint/BP_PlayerProto.BP_PlayerProto_C|GetFirstPersonCamera (Variables|Default|GetCachedCharacter)))) false false)
    (Rendering|Components|TextRender|SetText (Variables|Default|GetPingText) (Utilities|Text|ToText(String) (Class|KismetMathLibrary|FFloor64 (/ (Math|Vector|Distance(Vector) _returnvalue (Transformation|GetActorLocation (Variables|Default|GetCachedCharacter))) 1e+02))))))

(fn ConstructionScript)

(fn SetPingVisible
  (params (IsVisible :type Boolean))
  (bind _output_get (Variables|Default|SetIsPingVisible IsVisible))
  (Rendering|SetActorHiddenInGame (not _output_get)))