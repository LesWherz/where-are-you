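; BP_AC_Ping is an actor component on BP_PlayerProto that shows an on-screen ping widget for a pinged player.
; On BeginPlay it casts and stores its owner, then creates a W_Ping widget for player controller 0.
; Client_Ping passes the pinged player to the widget, adds it to the viewport, and removes it after DurationPing.
; CanPing allows a ping only while that widget is not in the viewport.
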(event Custom|Client_Ping
  (params (PingedPlayer :type BP%20Player%20Proto%20Object%20Reference))
  ;[1 1 1] Client_PlayerPing
  (Variables|/Game/Blueprints/BP_Ping/W_Ping.W_Ping_C|SetPingedPlayer (Variables|Default|GetPingWidget) PingedPlayer)
  (UserInterface|Viewport|AddtoViewport (Variables|Default|GetPingWidget) 0)
  (Utilities|FlowControl|Delay (Variables|Default|GetDurationPing))
  (Widget|RemovefromParent (Variables|Default|GetPingWidget)))

(event EventBeginPlay
  ;[1 1 1] Begin Play
  (bind _asbp_player_proto (Utilities|Casting|CastToBP_PlayerProto (Components|GetOwner self)))
  (Variables|Default|SetOwner _asbp_player_proto)
  (bind _returnvalue (UserInterface|CreateWidget "/Game/Blueprints/BP_Ping/W_Ping.W_Ping_C" (Game|GetPlayerController 0)))
  (Variables|Default|SetPingWidget _returnvalue))

(fn CanPing
  (return (not (UserInterface|Viewport|IsinViewport (Variables|Default|GetPingWidget)))))