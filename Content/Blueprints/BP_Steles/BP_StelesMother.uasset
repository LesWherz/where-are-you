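; Stele base Blueprint for a paired activation puzzle that opens tagged doors, usable only once IsActivateByLevelButton is set.
; Entering its box shows a hold-to-activate prompt; activation recolors cable and light, and leaving releases it.
; Cable changes, paired-stele checks and timer start/stop fan out through every PC_PlayerProto, mostly via Client calls.
; OpenTheDoor runs on authority, passing its gameplay tag to all BP_Door actors.
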(event OnComponentBeginOverlap(Box)
  (params (OverlappedComponent :type Primitive%20Component%20Object%20Reference) (OtherActor :type Actor%20Object%20Reference) (OtherComp :type Primitive%20Component%20Object%20Reference) (OtherBodyIndex :type Integer) (bFromSweep :type Boolean) (SweepResult :type Hit%20Result%20Structure%20%28by%20ref%29))
  ;[0 1 0.1018] PLAYER WALKING INSIDE THE STELE
  (if (Variables|Default|GetIsActivateByLevelButton)
    (if (not (Variables|Default|GetsomeoneInside))
      (Variables|Default|SetsomeoneInside true)
      ;;[1 1 1] Connecter pour test les stele
      (CallFunction|PlayerInsideEvent OtherActor))))

(event OnComponentEndOverlap(Box)
  (params (OverlappedComponent :type Primitive%20Component%20Object%20Reference) (OtherActor :type Actor%20Object%20Reference) (OtherComp :type Primitive%20Component%20Object%20Reference) (OtherBodyIndex :type Integer))
  ;[1 0.05671 0] PLAYER WALKING OUTSIDE THE STELE
  (if (Variables|Default|GetIsActivateByLevelButton)
    (if (Variables|Default|GetsomeoneInside)
      (Variables|Default|SetsomeoneInside false)
      (CallFunction|Releasing)
      (CallFunction|PlayerOutsideEvent OtherActor))))

(event Custom|OpenTheDoor
  ;[0.05044 1 0] OPEN THE DOOR
  (Networking|SwitchHasAuthority
    (:Authority
      (bind _outactors (Actor|GetAllActorsOfClass "/Game/Blueprints/BP_Door/BP_Door.BP_Door_C"))
      (for _array_element _outactors
        (Default|OpenDoorSTELE _array_element (Variables|Default|GetGamePlayTAGOpenDoor))))))

(event Custom|StopTimer
  ;[1 0.06091 0] PLAYER RELEASING STELE
  (bind _outactors (Actor|GetAllActorsOfClass "/Game/Assets/Character/Blueprint/PC_PlayerProto.PC_PlayerProto_C"))
  (for _array_element _outactors
    (Default|PCStopTimer _array_element)))

(event Custom|VerifNbrOfSteleActivated
  ;[0.03459 1 0] PLAYER ACTIVATE THE STELE
  (if (Variables|BP_StelesMother_C|GetIsActive? (Variables|Default|GetOtherStele))
    (bind _outactors (Actor|GetAllActorsOfClass "/Game/Assets/Character/Blueprint/PC_PlayerProto.PC_PlayerProto_C"))
    (for _array_element _outactors
      (Default|ClientPCStartTimer _array_element))))

(event Custom|PlayerOutsideEvent
  (params (Target :type Actor%20Object%20Reference))
  ;[1 0.05671 0] PLAYER WALKING OUTSIDE THE STELE
  (bind _aspc_player_proto (Utilities|Casting|CastToPC_PlayerProto (Game|GetInstigatorController Target)))
  (Default|ClientRemoveAllWidgetbyClass _aspc_player_proto "/Game/Blueprints/BP_Steles/W_HoldToActivate.W_HoldToActivate_C"))

(event Custom|Releasing
  ;[1 0.06091 0] PLAYER RELEASING STELE
  (if (Variables|Default|GetIsActivateByLevelButton)
    (bind _outactors (Actor|GetAllActorsOfClass "/Game/Assets/Character/Blueprint/PC_PlayerProto.PC_PlayerProto_C"))
    (for _array_element _outactors
      (Default|ClientChangeColor _array_element (Variables|Default|GetCableStele) "/Game/Blueprints/BP_Ping/M_Neon_InstRed.M_Neon_InstRed" self false))
    (CallFunction|StopTimer)))

(event Custom|Activating
  ;[0.03459 1 0] PLAYER ACTIVATE THE STELE
  (if (Variables|Default|GetIsActivateByLevelButton)
    (bind _outactors (Actor|GetAllActorsOfClass "/Game/Assets/Character/Blueprint/PC_PlayerProto.PC_PlayerProto_C"))
    (for _array_element _outactors
      (Default|ClientChangeColor _array_element (Variables|Default|GetCableStele) "/Game/Blueprints/BP_Ping/M_Neon_InstBlue.M_Neon_InstBlue" self true)
      (Rendering|Components|Light|SetLightColor (Variables|Default|GetPointLight) "(R=0.073712,G=1.000000,B=0.000000,A=1.000000)" true)
      (Default|ClientVerifNbrSteleActivated _array_element self))))

(event Custom|PlayerInsideEvent
  (params (Target :type Actor%20Object%20Reference))
  ;[0 1 0.1018] PLAYER WALKING INSIDE THE STELE
  (bind _aspc_player_proto (Utilities|Casting|CastToPC_PlayerProto (Game|GetInstigatorController Target)))
  (Default|ClientAddWidgetbyClass _aspc_player_proto "/Game/Blueprints/BP_Steles/W_HoldToActivate.W_HoldToActivate_C"))

(fn ConstructionScript)

(fn OnRepMaterial)