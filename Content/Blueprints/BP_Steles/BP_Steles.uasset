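; Co-op stele pair that opens a door when two players hold interact simultaneously, one in each of the left and right boxes.
; Overlaps record each side's player, and the authority shows or removes that client's hold-to-activate widget.
; Interact press and release route through the player's server RPC, as side setters update the held flags.
; Both flags start client timers on both players; releasing or leaving stops them.
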(event OnComponentBeginOverlap(Box_CollisionLeft)
  (params (OverlappedComponent :type Primitive%20Component%20Object%20Reference) (OtherActor :type Actor%20Object%20Reference) (OtherComp :type Primitive%20Component%20Object%20Reference) (OtherBodyIndex :type Integer) (bFromSweep :type Boolean) (SweepResult :type Hit%20Result%20Structure%20%28by%20ref%29))
  ;[1 1 1] Player enter in box collision
  (bind _bp_player (Utilities|IsPlayerColliding OtherActor OtherComp)
    (:True
      (Variables|Players|SetPlayerCollideLeft _bp_player)
      (Networking|SwitchHasAuthority
        (:Authority
          (Default|ClientAddWidgetbyClass _bp_player "/Game/Blueprints/BP_Steles/W_HoldToActivate.W_HoldToActivate_C"))))))

(event OnComponentEndOverlap(Box_CollisionLeft)
  (params (OverlappedComponent :type Primitive%20Component%20Object%20Reference) (OtherActor :type Actor%20Object%20Reference) (OtherComp :type Primitive%20Component%20Object%20Reference) (OtherBodyIndex :type Integer))
  ;[1 1 1] Player quit box collision
  (bind _bp_player (Utilities|IsPlayerColliding OtherActor OtherComp)
    (:True
      (CallFunction|StopTimerPlayers)
      (Variables|Players|SetPlayerCollideLeft 0)
      (Variables|Players|SetPlayerLeftHaveStartInteract false)
      (Networking|SwitchHasAuthority
        (:Authority
          (Default|ClientRemoveAllWidgetbyClass _bp_player "/Game/Blueprints/BP_Steles/W_HoldToActivate.W_HoldToActivate_C"))))))

(event OnComponentBeginOverlap(Box_CollisionRight)
  (params (OverlappedComponent :type Primitive%20Component%20Object%20Reference) (OtherActor :type Actor%20Object%20Reference) (OtherComp :type Primitive%20Component%20Object%20Reference) (OtherBodyIndex :type Integer) (bFromSweep :type Boolean) (SweepResult :type Hit%20Result%20Structure%20%28by%20ref%29))
  ;[1 1 1] Player enter in box collision
  (bind _bp_player (Utilities|IsPlayerColliding OtherActor OtherComp)
    (:True
      (Variables|Players|SetPlayerCollideRight _bp_player)
      (Networking|SwitchHasAuthority
        (:Authority
          (Default|ClientAddWidgetbyClass _bp_player "/Game/Blueprints/BP_Steles/W_HoldToActivate.W_HoldToActivate_C"))))))

(event OnComponentEndOverlap(Box_CollisionRight)
  (params (OverlappedComponent :type Primitive%20Component%20Object%20Reference) (OtherActor :type Actor%20Object%20Reference) (OtherComp :type Primitive%20Component%20Object%20Reference) (OtherBodyIndex :type Integer))
  ;[1 1 1] Player quit box collision
  (bind _bp_player (Utilities|IsPlayerColliding OtherActor OtherComp)
    (:True
      (CallFunction|StopTimerPlayers)
      (Variables|Players|SetPlayerCollideRight 0)
      (Variables|Players|SetPlayerRightHaveStartInteract false)
      (Networking|SwitchHasAuthority
        (:Authority
          (Default|ClientRemoveAllWidgetbyClass _bp_player "/Game/Blueprints/BP_Steles/W_HoldToActivate.W_HoldToActivate_C"))))))

(event Custom|CheckPlayersCanOpenDoor
  ;[1 1 1] Check if all Players interact and start or stop Timer
  (if (and (Variables|Players|GetPlayerLeftHaveStartInteract) (Variables|Players|GetPlayerRightHaveStartInteract))
    (CallFunction|StartTimerPlayers)
    (else
      (CallFunction|StopTimerPlayers))))

(event Custom|Interact%20Pressed
  (params (PlayerStartInteract :type BP%20Player%20Proto%20Object%20Reference))
  (bind _self self)
  ;[1 1 1] Player Input Interract
  (Utilities|PlayerInteractIsPlayertoComparate PlayerStartInteract (Variables|Players|GetPlayerCollideLeft)
    (:True
      (Default|ServerSavePlayerInteractStele PlayerStartInteract _self true true))
    (:False
      (Utilities|PlayerInteractIsPlayertoComparate PlayerStartInteract (Variables|Players|GetPlayerCollideRight)
        (:True
          (Default|ServerSavePlayerInteractStele PlayerStartInteract _self false true))))))

(event Custom|Interact%20Released
  (params (PlayerEndInteract :type BP%20Player%20Proto%20Object%20Reference))
  (bind _self self)
  ;[1 1 1] Player Input Interract
  (Utilities|PlayerInteractIsPlayertoComparate PlayerEndInteract (Variables|Players|GetPlayerCollideLeft)
    (:True
      (Default|ServerSavePlayerInteractStele PlayerEndInteract _self true false))
    (:False
      (Utilities|PlayerInteractIsPlayertoComparate PlayerEndInteract (Variables|Players|GetPlayerCollideRight)
        (:True
          (Default|ServerSavePlayerInteractStele PlayerEndInteract _self false false))))))

(event Custom|SetPlayerLeftInteract
  (params (HaveStart :type Boolean))
  ;[1 1 1] Set Players Interact
  (Variables|Players|SetPlayerLeftHaveStartInteract HaveStart)
  (CallFunction|CheckPlayersCanOpenDoor))

(event Custom|SetPlayerRightInteract
  (params (HaveStart :type Boolean))
  ;[1 1 1] Set Players Interact
  (Variables|Players|SetPlayerRightHaveStartInteract HaveStart)
  (CallFunction|CheckPlayersCanOpenDoor))

(fn ConstructionScript)

(fn StartTimerPlayers
  (Default|ClientStartTimerStele (Variables|Players|GetPlayerCollideLeft))
  (Default|ClientStartTimerStele (Variables|Players|GetPlayerCollideRight)))

(fn StopTimerPlayers
  (bind _playercollideleft (Variables|Players|GetPlayerCollideLeft))
  (bind _playercollideright (Variables|Players|GetPlayerCollideRight))
  (Utilities|IsValid _playercollideleft
    (:Is%20Valid
      (Default|ClientStopTimerStele _playercollideleft))
    (:Is%20Not%20Valid
      _))
  (Utilities|IsValid _playercollideright
    (:Is%20Valid
      (Default|ClientStopTimerStele _playercollideright))))