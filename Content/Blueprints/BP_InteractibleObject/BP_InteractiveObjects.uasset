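; Networked interactive object that steps between Small, Normal and Big sizes.
; Server resize events route through BP_PlayerProto, with growth gated by box traces against static world, heightened for any player in the target volume.
; Client_ResizeObject lerps scale in a Delay loop under a Resizing state, with start/end hooks driving material VFX and sound.
; The construction script caches bounds for those traces and a query-only box enabled when Small.
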(event Custom|Server_ResizeObjectSmaller
  ;[0.574 0.7082 1] Make object smaller / bigger events
  (switch Utilities|FlowControl|Switch|SwitchonEObjectSizeState (Variables|Default|GetResizableObjectState)
    (:Normal
      (Variables|Default|SetResizableObjectState "Small"))
    (:Big
      (Variables|Default|SetResizableObjectState "Normal")))
  (bind _asbp_player_proto (Utilities|Casting|CastToBP_PlayerProto (Game|Player|GetPlayerPawn 0)))
  (Default|ServerResizeObject _asbp_player_proto self (Variables|Default|GetResizableObjectState)))

(event Custom|Server_ResizeObjectBigger
  ;[0.574 0.7082 1] Make object smaller / bigger events
  (switch Utilities|FlowControl|Switch|SwitchonEObjectSizeState (Variables|Default|GetResizableObjectState)
    (:Small
      (Utilities|CanResize "Normal"
        (:ResizeWillSuceed
          (Variables|Default|SetResizableObjectState "Normal")
          (bind _asbp_player_proto (Utilities|Casting|CastToBP_PlayerProto (Game|Player|GetPlayerPawn 0) :!label _label))
          (Default|ServerResizeObject _asbp_player_proto self (Variables|Default|GetResizableObjectState)))
        (:ResizeWillFail
          (Development|PrintString "Can not resize" :!label _label_2))))
    (:Normal
      (Utilities|CanResize "Big"
        (:ResizeWillSuceed
          (Variables|Default|SetResizableObjectState "Big")
          (goto _label))
        (:ResizeWillFail
          (goto _label_2))))))

(event Custom|Client_ResizeObject
  (params (State :type EObjectSizeState%20Enum :default "Resizing"))
  (if (not (Utilities|Enum|Equal(Enum) (Variables|Default|GetResizableObjectState) "Resizing"))
    ;[0.8245 1 0.7615] Initialization
    (Variables|Lerp|SetStartScaleFactor (.x (Transformation|GetWorldScale (Variables|Transformation|GetRootComponent))))
    (bind _output_get (Variables|Default|SetResizableObjectState State))
    (switch Utilities|FlowControl|Switch|SwitchonEObjectSizeState _output_get
      (:Small
        (Variables|Lerp|SetTargetScaleFactor (Variables|Default|GetSmallScaleFactor)))
      (:Normal
        (Variables|Lerp|SetTargetScaleFactor (Variables|Default|GetNormalScaleFactor)))
      (:Big
        (Variables|Lerp|SetTargetScaleFactor (Variables|Default|GetBigScaleFactor))))
    (Utilities|FlowControl|Sequence
      (:then_0
        (Variables|Default|SetTempResizableObjectState (Variables|Default|GetResizableObjectState))
        (Variables|Default|SetResizableObjectState "Resizing"))
      (:then_1
        (CallFunction|OnResizeStart (Variables|Default|GetTempResizableObjectState) (> (Variables|Lerp|GetStartScaleFactor) (Variables|Lerp|GetTargetScaleFactor))))
      (:then_2
        ;[1 0.6352 0.9897] Lerp Resize
        (Variables|Lerp|SetTimeLerpResize 0.0)
        (if (< (Variables|Lerp|GetTimeLerpResize) (Variables|Lerp|GetDurationLerpResize)) :!label _label
          (CallFunction|SetNewWorldScale (Math|Float|Lerp (Variables|Lerp|GetStartScaleFactor) (Variables|Lerp|GetTargetScaleFactor) (/ (Variables|Lerp|GetTimeLerpResize) (Variables|Lerp|GetDurationLerpResize))))
          (Utilities|FlowControl|Delay (Variables|Default|GetDeltaTime))
          (Variables|Lerp|SetTimeLerpResize (+ (Variables|Lerp|GetTimeLerpResize) (Variables|Default|GetDeltaTime)))
          (goto _label)
          (else
            (CallFunction|SetNewWorldScale (Variables|Lerp|GetTargetScaleFactor))
            (bind _output_get_2 (Variables|Default|SetResizableObjectState (Variables|Default|GetTempResizableObjectState)))
            (CallFunction|OnResizeEnd _output_get_2)))))))

(event EventBeginPlay
  ;[1 1 1] BeginPlay
  (Utilities|FlowControl|Sequence
    (:then_0
      ;;[1 1 1] Setup Id
      (bind _asbp_player_proto (Utilities|Casting|CastToBP_PlayerProto (Game|GetPlayerCharacter 0)))
      (Default|ClientSetupResizableId _asbp_player_proto self))
    (:then_1
      (bind _aspc_player_proto (Utilities|Casting|CastToPC_PlayerProto (Game|GetPlayerController 0)))
      (Variables|Default|SetPlayerControllerRef _aspc_player_proto))
    (:then_2
      (CallFunction|UpdateShrunkedBoxCollisionComp (Variables|Default|GetResizableObjectState)))
    (:then_3
      (if (Utilities|Enum|Equal(Enum) (Variables|Default|GetResizableObjectState) "Resizing")
        (Development|PrintString "One of your objects in in state \"Resizing\". Switching to \"Normal.\"" true true "(R=1.000000,G=0.000000,B=0.000000,A=1.000000)" 5.0)
        (CallFunction|SetNewWorldScale (Variables|Default|GetNormalScaleFactor))
        (Variables|Default|SetResizableObjectState "Normal")))))

(event EventTick
  (params (DeltaSeconds :type Float%20%28single-precision%29))
  ;[1 1 1] Update deltaTime
  (Variables|Default|SetDeltaTime DeltaSeconds))

(fn ConstructionScript
  (bind _sm_object (Variables|Default|GetSM_Object))
  (bind _sm_object_2 (Variables|Default|GetSM_Object))
  (bind (_origin _boxextent) (Collision|GetComponentBounds _sm_object))
  (Utilities|FlowControl|Sequence
    (:then_0
      (Utilities|FlowControl|Sequence
        (:then_0
          (bind _scalefactor (CallFunction|GetScaleFactorforResizeState (Variables|Default|GetResizableObjectState)))
          (CallFunction|SetNewWorldScale (Variables|Default|GetNormalScaleFactor)))
        (:then_1
          (Variables|ResizeTests|SetBaseSMWorldOrigin _origin)
          (bind _output_get (Variables|ResizeTests|SetBaseSMBoxExtent (* _boxextent (Variables|ResizeTests|GetBoxExtentRatioForResizeTests))))
          (Components|Box|SetBoxExtent (Variables|Default|GetShrunkedBoxCollision) _output_get true)
          (Variables|ResizeTests|SetShrunkedBoxCollisionBoxExtent (* _boxextent (Variables|ResizeTests|GetShrunkedBoxColSizeFactor))))
        (:then_2
          (CallFunction|SetNewWorldScale _scalefactor)
          (CallFunction|UpdateShrunkedBoxCollisionComp (Variables|Default|GetResizableObjectState)))))
    (:then_1
      (bind _returnvalue (Rendering|Material|CreateDynamicMaterialInstance _sm_object_2 0 (Rendering|Material|GetMaterial _sm_object_2 0) "None" :!class /Script/Engine.PrimitiveComponent))
      (Rendering|Material|SetMaterial (Variables|Default|GetSM_Object) 0 _returnvalue)
      (Variables|Default|SetCurrent%20Dynamic%20Material _returnvalue))))

(fn SetNewWorldScale
  (params (newScaleFactor :type Float%20%28single-precision%29))
  (Transformation|SetWorldScale3D (Variables|Transformation|GetRootComponent) (Math|Conversions|ToVector(Float) newScaleFactor)))

(fn OnRepResizableObjectState)

(fn OnRepTimeLerpResize)

(fn GetScaleFactorforResizeState
  (params (ResizeState :type EObjectSizeState%20Enum :default "Resizing"))
  (switch Utilities|FlowControl|Switch|SwitchonEObjectSizeState ResizeState
    (:Small
      (return (Variables|Default|GetSmallScaleFactor)))
    (:Normal
      (return (Variables|Default|GetNormalScaleFactor)))
    (:Big
      (return (Variables|Default|GetBigScaleFactor)))
    (:Resizing
      (Development|PrintString "Trying to get scale factor while resizing..."))))

(fn UpdateShrunkedBoxCollisionComp
  (params (InObjectState :type EObjectSizeState%20Enum :default "Resizing"))
  (bind _shrunkedboxcollision (Variables|Default|GetShrunkedBoxCollision))
  (if (Utilities|Enum|NotEqual(Enum) InObjectState "Small")
    (Collision|SetCollisionEnabled _shrunkedboxcollision "NoCollision")
    (else
      (Collision|SetCollisionEnabled _shrunkedboxcollision "QueryOnly")
      (Components|Box|SetBoxExtent (Variables|Default|GetShrunkedBoxCollision) (* (Variables|ResizeTests|GetShrunkedBoxCollisionBoxExtent) (/ (Variables|Default|GetNormalScaleFactor) (Variables|Default|GetSmallScaleFactor))) true)
      (Transformation|SetWorldLocation (Variables|Default|GetShrunkedBoxCollision) (Utilities|GetOffsetedSMWorldOriginforScaleFactor (Variables|ResizeTests|GetShrunkedBoxColSizeFactor)) false false))))

(fn OnResizeStart
  (params (FutureSizeState :type EObjectSizeState%20Enum :default "Resizing") (WillGrowingUp :type Boolean))
  (bind _playercontrollerref (Variables|Default|GetPlayerControllerRef))
  (bind _sm_object (Variables|Default|GetSM_Object))
  (bind _current_dynamic_material (Variables|Default|GetCurrent%20Dynamic%20Material))
  (Utilities|FlowControl|Sequence
    (:then_0
      ;[1 1 1] System
      (CallFunction|UpdateShrunkedBoxCollisionComp "Resizing"))
    (:then_1
      ;[1 1 1] VFX
      (Rendering|Material|SetScalarParameterValuebyInfo _current_dynamic_material (Utilities|Struct|MakeMaterialParameterInfo "CTRL_VFXReduc" "LayerParameter" 1) 1.0)
      (Rendering|Material|SetScalarParameterValuebyInfo _current_dynamic_material (Utilities|Struct|MakeMaterialParameterInfo "CTRL_VFXReduc" "BlendParameter" 0) 1.0)
      (Class|MaterialInstanceDynamic|SetVectorParameterValuebyInfo _current_dynamic_material (Utilities|Struct|MakeMaterialParameterInfo "GlobalColor" "LayerParameter" 1) (select (not WillGrowingUp) "(R=0.000000,G=60.000000,B=0.000000,A=1.000000)" "(R=60.000000,G=0.000000,B=0.000000,A=1.000000)")))
    (:then_2
      ;[1 1 1] Sounds
      (if WillGrowingUp
        (Default|OwnClientSpawnSoundAttached _playercontrollerref "/Game/StarterContent/Audio/Explosion01.Explosion01" _sm_object "SnapToTarget" 0 0 true)
        (else
          (Default|OwnClientSpawnSoundAttached _playercontrollerref "/Game/StarterContent/Audio/Explosion02.Explosion02" _sm_object "SnapToTarget" 0 0 true))))))

(fn OnResizeEnd
  (params (CurrentSizeState :type EObjectSizeState%20Enum :default "Resizing"))
  (bind _current_dynamic_material (Variables|Default|GetCurrent%20Dynamic%20Material))
  (Utilities|FlowControl|Sequence
    (:then_0
      ;[1 1 1] System
      (CallFunction|UpdateShrunkedBoxCollisionComp CurrentSizeState))
    (:then_1
      ;[1 1 1] VFX
      (Rendering|Material|SetScalarParameterValuebyInfo _current_dynamic_material (Utilities|Struct|MakeMaterialParameterInfo "CTRL_VFXReduc" "LayerParameter" 1) 0.0)
      (Rendering|Material|SetScalarParameterValuebyInfo _current_dynamic_material (Utilities|Struct|MakeMaterialParameterInfo "CTRL_VFXReduc" "BlendParameter" 0) 0.0)
      (Rendering|Material|SetScalarParameterValuebyInfo _current_dynamic_material (Utilities|Struct|MakeMaterialParameterInfo "CTRL_VFXReduc" "BlendParameter" 0) 0.0)
      (Class|MaterialInstanceDynamic|SetVectorParameterValuebyInfo _current_dynamic_material (Utilities|Struct|MakeMaterialParameterInfo "GlobalColor" "LayerParameter" 1) "(R=60.000000,G=60.000000,B=0.000000,A=1.000000)"))))