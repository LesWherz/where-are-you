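; BP_Laser is a laser effect actor that fires a red beam along its forward direction until it hits something.
; On BeginPlay it sets an overbright red color parameter on the beam and impact effects.
; Each tick it runs a very long Visibility line trace and feeds the beam's begin and end parameters from it.
; The impact effect follows the hit location and shows only on a blocking hit.
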(event EventBeginPlay
  (Effects|Components|ParticleSystem|SetColorParameter (Variables|Default|Getlaser) "Color" "(R=30.000000,G=0.000000,B=0.000000,A=1.000000)"))

(event EventTick
  (params (DeltaSeconds :type Float%20%28single-precision%29))
  (bind _returnvalue (Transformation|GetActorLocation))
  (bind _laser (Variables|Default|Getlaser))
  (bind _laserimpact (Variables|Default|GetlaserImpact))
  (bind _outhit (Collision|LineTraceByChannel _returnvalue (+ _returnvalue (* (Transformation|GetActorForwardVector) 2e+09)) "TraceTypeQuery1" false 0 "None"))
  (Effects|Components|ParticleSystem|SetVectorParameter _laser "LaserBegin" _returnvalue)
  (Effects|Components|ParticleSystem|SetVectorParameter _laser "LaserEnd" (select (.bblockinghit _outhit) (.location _outhit) (Variables|Default|GetTraceEnd)))
  (Rendering|SetVisibility _laserimpact (.bblockinghit _outhit) false)
  (Transformation|SetWorldLocation _laserimpact (.location _outhit) false false))

(fn ConstructionScript)