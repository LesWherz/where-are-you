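; HUD_PlayerProto is a prototype player HUD that draws a crosshair near the screen center.
; Each DrawHUD event passes the screen size to Draw Mire, which skips drawing when a head-mounted display is enabled.
; Otherwise it offsets the CrossHair texture from the center by half its native size and draws it at a fixed 16x16 size.
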(event EventDrawHUD
  (params (SizeX :type Integer) (SizeY :type Integer))
  (Utilities|FlowControl|Sequence
    (:then_0
      (|DrawMire SizeX SizeY))))

(fn ConstructionScript)