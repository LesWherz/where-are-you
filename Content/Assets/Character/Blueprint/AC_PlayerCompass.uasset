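; Player compass component that shows a HUD arrow pointing toward the other player.
; On BeginPlay it caches the BP_PlayerProto owner and creates the W_HUDCompass widget through an OwnClient event.
; Each Tick rotates the arrow using the 2D angle between camera forward and the inter-player vector, signed by a cross product.
; Arrow size follows player distance through a clamped range mapping.
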(event Custom|OwnClient_CreateHUDCompass
  ;[1 1 1] Create HUD compass
  (bind _aspc_player_proto (Utilities|Casting|CastToPC_PlayerProto (Game|GetInstigatorController (Variables|Default|GetPlayerOwner))))
  (bind _returnvalue (UserInterface|CreateWidget "/Game/Assets/UI/Widgets/W_HUDCompass.W_HUDCompass_C" _aspc_player_proto))
  (UserInterface|Viewport|AddtoViewport _returnvalue 0)
  (Variables|Default|SetW_HUDCompass_Ref _returnvalue))

(event Custom|OwnClient_UpdateHUDCompass
  (bind _playerowner (Variables|Default|GetPlayerOwner))
  (bind _arrowminscale (Variables|Default|GetArrowMinScale))
  (bind _arrowmaxscale (Variables|Default|GetArrowMaxScale))
  (bind _playerowner_2 (Variables|Default|GetPlayerOwner))
  (bind _playerowner_3 (Variables|Default|GetPlayerOwner))
  (bind _distanceforarrowminsize (Variables|Default|GetDistanceForArrowMinSize))
  (bind _distanceforarrowmaxsize (Variables|Default|GetDistanceForArrowMaxSize))
  (bind _playerowner_4 (Variables|Default|GetPlayerOwner))
  (bind _returnvalue (Transformation|GetActorLocation _playerowner))
  (bind _otherplayer (Variables|/Game/Assets/Character/Blueprint/BP_PlayerProto.BP_PlayerProto_C|GetOtherPlayer _playerowner_3))
  (bind _firstpersoncamera (Variables|/Game/Assets/Character/Blueprint/BP_PlayerProto.BP_PlayerProto_C|GetFirstPersonCamera _playerowner))
  (bind _otherplayer_2 (Variables|/Game/Assets/Character/Blueprint/BP_PlayerProto.BP_PlayerProto_C|GetOtherPlayer _playerowner_4))
  (bind _returnvalue_2 (Transformation|GetDistanceTo _playerowner_2 _otherplayer))
  (bind _returnvalue_3 (Math|Vector|GetForwardVector _firstpersoncamera))
  (bind _returnvalue_4 (Transformation|GetActorLocation _otherplayer_2))
  (bind _returnvalue_5 (- _returnvalue _returnvalue_4))
  (bind _returnvalue_6 (Math|Float|MapRangeClamped _returnvalue_2 _distanceforarrowminsize _distanceforarrowmaxsize _arrowmaxscale _arrowminscale))
  (bind _returnvalue_7 (Class|KismetMathLibrary|VectorCosineAngle2D _returnvalue_3 _returnvalue_5))
  (bind _returnvalue_8 (Math|Trig|Acos(Degrees) _returnvalue_7))
  (bind _returnvalue_9 (Math|Trig|RadiansToDegrees _returnvalue_8))
  (bind _returnvalue_10 (- _returnvalue_9 1.8e+02))
  ;[1 1 1] Update arrow angle, based on other player position
  (if (and (Utilities|IsValid (Variables|/Game/Assets/Character/Blueprint/BP_PlayerProto.BP_PlayerProto_C|GetOtherPlayer (Variables|Default|GetPlayerOwner))) (Utilities|IsValid (Variables|Default|GetW_HUDCompass_Ref)))
    (Class|Widget|SetRenderTransformAngle (Variables|/Game/Assets/UI/Widgets/W_HUDCompass.W_HUDCompass_C|GetCANVAS_ParentArrow (Variables|Default|GetW_HUDCompass_Ref)) (Math|Float|SelectFloat _returnvalue_10 (* _returnvalue_10 -1.0) (> (Class|KismetMathLibrary|CrossProduct2D (Math|Conversions|ToVector2D(Vector) _returnvalue_3) (Math|Conversions|ToVector2D(Vector) _returnvalue_5)) 0.0)))
    ;[1 1 1] Set arrow scale, based on distance from other player
    (Class|CanvasPanelSlot|SetSize (Class|WidgetLayoutLibrary|SlotasCanvasSlot (Variables|/Game/Assets/UI/Widgets/W_HUDCompass.W_HUDCompass_C|GetIMG_Arrow (Variables|Default|GetW_HUDCompass_Ref))) (Math|Vector2D|MakeVector2D _returnvalue_6 _returnvalue_6))))

(event EventBeginPlay
  (Utilities|FlowControl|Sequence
    (:then_0
      ;[1 1 1] Get the player owner
      (bind _asbp_player_proto (Utilities|Casting|CastToBP_PlayerProto (Components|GetOwner self)))
      (Variables|Default|SetPlayerOwner _asbp_player_proto))
    (:then_1
      ;[1 1 1] Create HUD compass
      (CallFunction|OwnClientCreateHUDCompass))))

(event EventTick
  (params (DeltaSeconds :type Float%20%28single-precision%29))
  ;[1 1 1] Udate compass
  (CallFunction|OwnClientUpdateHUDCompass))