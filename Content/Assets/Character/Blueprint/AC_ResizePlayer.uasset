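; Player component that toggles BP_PlayerProto between normal and shrunk size.
; Client_ResizePlayer lerps the capsule's world scale through a frame-delta Delay loop, holding a Resizing state until done.
; Begin and end hooks update collision profile, step height, floor offset, movement, object aiming, material FX, Cerclage visibility and sound.
; CanGrowUp uses line and capsule traces to check headroom, but is not called here.
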(event Custom|Client_ResizePlayer
  ;[1 1 1] Client_ResizePlayer : Initialisation
  (switch Utilities|FlowControl|Switch|SwitchonEPlayerSizeState (Variables|Default|GetPlayerSizeState)
    (:Normal
      (Variables|Default|SetPlayerSizeState "Shrunked")
      (Variables|PlayerSizeCalculation|SetTargetScaleFactor (Variables|Default|GetShrunkedScaleFactor))
      (Variables|PlayerSizeCalculation|SetTargetCapsuleRadius (Variables|Default|GetShunkedCapsuleRadius)))
    (:Shrunked
      (Variables|Default|SetPlayerSizeState "Normal")
      (Variables|PlayerSizeCalculation|SetTargetScaleFactor 1.0)
      (Variables|PlayerSizeCalculation|SetTargetCapsuleRadius (Variables|PlayerSizeCalculation|GetNormalCapsuleRadius))))
  (Utilities|FlowControl|Sequence
    (:then_0
      (Variables|Default|SetPlayerSizeStateBeforeResize (Variables|Default|GetPlayerSizeState)))
    (:then_1
      (Variables|Default|SetPlayerSizeState "Resizing"))
    (:then_2
      (CallFunction|OnResizeBegin (Variables|Default|GetPlayerSizeStateBeforeResize)))
    (:then_3
      ;[1 1 1] Client_ResizePlayer : Lerp Resize
      (Variables|Default|SetTimeLerpResize 0.0)
      (if (< (Variables|Default|GetTimeLerpResize) (Variables|Default|GetDurationLerpResize)) :!label _label
        (|SetNewLerpedScale (/ (Variables|Default|GetTimeLerpResize) (Variables|Default|GetDurationLerpResize)))
        (Utilities|FlowControl|Delay (Variables|Default|GetDeltaTime))
        (Variables|Default|SetTimeLerpResize (+ (Variables|Default|GetTimeLerpResize) (Variables|Default|GetDeltaTime)))
        (goto _label)
        (else
          ;[1 1 1] Client_ResizePlayer : Resize end. Update player size state
          (Variables|PlayerSizeCalculation|SetPlayerScaleFactor (Variables|PlayerSizeCalculation|GetTargetScaleFactor))
          (Transformation|SetWorldScale3D (Variables|/Script/Engine.Character|GetCapsuleComponent (Variables|Default|GetOwner)) (Math|Vector|MakeVector (Variables|PlayerSizeCalculation|GetPlayerScaleFactor) (Variables|PlayerSizeCalculation|GetPlayerScaleFactor) (Variables|PlayerSizeCalculation|GetPlayerScaleFactor)))
          (Variables|Default|SetPlayerSizeState (Variables|Default|GetPlayerSizeStateBeforeResize))
          (CallFunction|OnResizeEnd (Variables|Default|GetPlayerSizeState)))))))

(event EventBeginPlay
  (Utilities|FlowControl|Sequence
    (:then_0
      ;[1 1 1] Get the player owner
      (bind _asbp_player_proto (Utilities|Casting|CastToBP_PlayerProto (Components|GetOwner self)))
      (Variables|Default|SetOwner _asbp_player_proto))
    (:then_1
      ;[1 1 1] Resize Init
      (bind _output_get (Variables|PlayerSizeCalculation|SetNormalCapsuleHeight (* (Variables|/Script/Engine.CapsuleComponent|GetCapsuleHalfHeight (Variables|/Script/Engine.Character|GetCapsuleComponent (Variables|Default|GetOwner))) 2.0)))
      (Variables|PlayerSizeCalculation|SetShrunkedCapsuleHeight (* _output_get (Variables|Default|GetShrunkedScaleFactor)))
      (Variables|PlayerSizeCalculation|SetNormalCapsuleRadius (Variables|/Script/Engine.CapsuleComponent|GetCapsuleRadius (Variables|/Script/Engine.Character|GetCapsuleComponent (Variables|Default|GetOwner)))))))

(event EventTick
  (params (DeltaSeconds :type Float%20%28single-precision%29))
  ;[1 1 1] DeltaTimeUpdate
  (Variables|Default|SetDeltaTime DeltaSeconds))

(fn CanGrowUp
  (bind _shrunkedcapsuleheight (Variables|PlayerSizeCalculation|GetShrunkedCapsuleHeight))
  (bind _owner (Variables|Default|GetOwner))
  (bind _normalcapsuleheight (Variables|PlayerSizeCalculation|GetNormalCapsuleHeight))
  (bind _normalcapsuleradius (Variables|PlayerSizeCalculation|GetNormalCapsuleRadius))
  (bind _normalcapsuleradius_2 (Variables|PlayerSizeCalculation|GetNormalCapsuleRadius))
  (bind _returnvalue (/ _shrunkedcapsuleheight 2.0))
  (bind _capsulecomponent (Variables|/Script/Engine.Character|GetCapsuleComponent _owner))
  (bind _returnvalue_2 (Transformation|GetWorldLocation _capsulecomponent))
  (bind _returnvalue_3 (+ (.z _returnvalue_2) _returnvalue))
  (bind _returnvalue_4 (+ _returnvalue_3 _normalcapsuleheight))
  (bind _returnvalue_5 (+ _normalcapsuleradius_2 _returnvalue_3))
  (bind _returnvalue_6 (Math|Vector|MakeVector (.x _returnvalue_2) (.y _returnvalue_2) _returnvalue_5))
  (bind _returnvalue_7 (- _returnvalue_4 _normalcapsuleradius))
  (bind _returnvalue_8 (Math|Vector|MakeVector (.x _returnvalue_2) (.y _returnvalue_2) _returnvalue_7))
  (bind _returnvalue_9 (Collision|LineTraceByChannel _returnvalue_6 _returnvalue_8 "TraceTypeQuery1" false 0 "None"))
  (if (not _returnvalue_9)
    (bind _returnvalue_10 (Collision|CapsuleTraceByChannel _returnvalue_6 _returnvalue_8 (* (Variables|PlayerSizeCalculation|GetNormalCapsuleRadius) (Variables|Default|GetGrowUpCollisionCheckRadiusFactor)) 0.0 "TraceTypeQuery1" false 0 "None"))
    (return (not _returnvalue_10))
    (else
      (return false))))

(fn Construction)

(fn OnResizeBegin
  (params (FutureSizeState :type EPlayerSizeState%20Enum :default "Normal"))
  (bind _owner (Variables|Default|GetOwner))
  (bind _owner_2 (Variables|Default|GetOwner))
  (bind _owner_3 (Variables|Default|GetOwner))
  (bind _owner_4 (Variables|Default|GetOwner))
  (bind _capsulecomponent (Variables|/Script/Engine.Character|GetCapsuleComponent _owner_4))
  (bind _charactermovement (Variables|/Script/Engine.Character|GetCharacterMovement _owner_3))
  (Utilities|FlowControl|Sequence
    (:then_0
      (Utilities|FlowControl|Sequence
        (:then_0
          (Default|UpdateShrunkedCollisionCompActivation (Variables|Default|GetOwner) true))
        (:then_1
          ;[1 1 1] Update collision and step height behaviour
          (if (Utilities|Enum|Equal(Enum) FutureSizeState "Shrunked")
            (Collision|SetCollisionProfileName _capsulecomponent "ShrunkedPawn" true :!class /Script/Engine.PrimitiveComponent)
            (Variables|/Script/Engine.CharacterMovementComponent|SetMaxStepHeight _charactermovement 0.0)
            (else
              (Collision|SetCollisionProfileName _capsulecomponent "Pawn" true :!class /Script/Engine.PrimitiveComponent)
              (Variables|/Script/Engine.CharacterMovementComponent|SetMaxStepHeight _charactermovement (Variables|/Game/Assets/Character/Blueprint/BP_PlayerProto.BP_PlayerProto_C|GetBaseMaxWalkStepHeight _owner_3)))))
        (:then_2
          ;[1 1 1] Update player floor offset (to not see the model flying above the ground when Shurnked)
          (if (Utilities|Enum|Equal(Enum) FutureSizeState "Normal")
            (Default|UpdateFloorOffset (Variables|Default|GetOwner) true)
            (Default|TryStopAimingCurrentObject (Variables|/Game/Assets/Character/Blueprint/BP_PlayerProto.BP_PlayerProto_C|GetAC_PlayerObjectHighlight (Variables|Default|GetOwner)))))))
    (:then_1
      (Utilities|FlowControl|Sequence
        (:then_0
          (CallFunction|FXResizeCharacter FutureSizeState false))
        (:then_1
          (if (Utilities|Enum|Equal(Enum) FutureSizeState "Normal")
            (Default|OwnClientSpawnSoundAttached (Variables|/Game/Assets/Character/Blueprint/BP_PlayerProto.BP_PlayerProto_C|GetPlayerControllerRef _owner_2) "/Game/Sounds/SFX_Tir_Neutral.SFX_Tir_Neutral" (Variables|/Script/Engine.Character|GetCapsuleComponent _owner_2) "SnapToTarget" 0 0 true)
            (else
              (Default|OwnClientSpawnSoundAttached (Variables|/Game/Assets/Character/Blueprint/BP_PlayerProto.BP_PlayerProto_C|GetPlayerControllerRef _owner) "/Game/Sounds/SFX_Tir_Shrink.SFX_Tir_Shrink" (Variables|/Script/Engine.Character|GetCapsuleComponent _owner) "SnapToTarget" 0 0 true))))))))

(fn OnResizeEnd
  (params (CurrPlayerSizeState :type EPlayerSizeState%20Enum :default "Normal"))
  (bind _owner (Variables|Default|GetOwner))
  (Utilities|FlowControl|Sequence
    (:then_0
      (Default|UpdatePlayerMovementParameters (Variables|Default|GetOwner))
      (Default|UpdateShrunkedCollisionCompActivation (Variables|Default|GetOwner) false)
      (if (Utilities|Enum|Equal(Enum) (Variables|AC_ResizePlayer_C|GetPlayerSizeState (Variables|/Game/Assets/Character/Blueprint/BP_PlayerProto.BP_PlayerProto_C|GetAC_ResizePlayer (Variables|Default|GetOwner))) "Shrunked")
        (Default|TryStopAimingCurrentObject (Variables|/Game/Assets/Character/Blueprint/BP_PlayerProto.BP_PlayerProto_C|GetAC_PlayerObjectHighlight (Variables|Default|GetOwner)))))
    (:then_1
      (if (Utilities|Enum|Equal(Enum) CurrPlayerSizeState "Shrunked")
        (Default|UpdateFloorOffset _owner false)))
    (:then_2
      (CallFunction|FXResizeCharacter "Normal" true)
      (Rendering|SetVisibility (Variables|/Game/Assets/Character/Blueprint/BP_PlayerProto.BP_PlayerProto_C|GetCerclage _owner) (Utilities|Select :Index CurrPlayerSizeState :Normal false :Shrunked true :Resizing false) false))))

(fn FXResizeCharacter
  (params (Future%20size%20state :type EPlayerSizeState%20Enum :default "Normal") (Set%20to%200 :type Boolean))
  (bind _owner (Variables|Default|GetOwner))
  (Rendering|Material|SetScalarParameterValue (Variables|/Game/Assets/Character/Blueprint/BP_PlayerProto.BP_PlayerProto_C|GetCurrent%20Material _owner) "Switch_Modes" (select Set%20to%200 0.0 (Utilities|Select :Index Future%20size%20state :Normal 2.0 :Shrunked 1.0 :Resizing 0.0)) :!class /Script/Engine.MaterialInstanceDynamic)
  (Rendering|SetVisibility (Variables|/Game/Assets/Character/Blueprint/BP_PlayerProto.BP_PlayerProto_C|GetCerclage _owner) false false))