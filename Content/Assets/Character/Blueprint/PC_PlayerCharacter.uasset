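; PC_PlayerCharacter is a player controller that relays puzzle interactions to steles and digicodes and handles leaving the online session.
; Its events cast incoming actors to set stele cable materials and active state, check the activated stele count, or pass digicode button input.
; Timer events start and end the hold-to-activate widget's countdown.
; A successful session destroy triggers ejecting the player from the player list.
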(event EventBeginPlay)

(event EventTick
  (params (DeltaSeconds :type Float%20%28single-precision%29)))

(event EventChangeColorCableStele
  (params (Cable :type Actor%20Object%20Reference) (Material :type Material%20Interface%20Object%20Reference) (Stele :type Actor%20Object%20Reference) (IsActive :type Boolean))
  (bind _asbp_cable_for_stele (Utilities|Casting|CastToBP_CableForStele Cable))
  (Rendering|Material|SetMaterial (Variables|/Game/Blueprints/BP_Steles/BP_CableForStele.BP_CableForStele_C|GetCable _asbp_cable_for_stele) 0 Material)
  (bind _asbp_steles_mother (Utilities|Casting|CastToBP_StelesMother Stele))
  (Variables|/Game/Blueprints/BP_Steles/BP_StelesMother.BP_StelesMother_C|SetIsActive? _asbp_steles_mother IsActive))

(event EventChangeTextDigicode
  (params (Digicode :type Actor%20Object%20Reference) (Text :type String))
  (bind _asbp_digicode (Utilities|Casting|CastToBP_Digicode Digicode))
  (Default|OnButtonPressed _asbp_digicode Text))

(event EventClientPCStartTimer
  (bind _asw_hold_to_activate (Utilities|Casting|CastToW_HoldToActivate (Variables|Default|GetmyWidget)))
  (Development|PrintString "START TIMER" true true "(R=0.000000,G=0.660000,B=1.000000,A=1.000000)" 1e+01)
  (Default|StartTimer _asw_hold_to_activate))

(event EventDestroySession
  (|DestroySession self
    (:OnSuccess
      (Class|PCPlayerCharacter|EjectPlayerfromPlayerList))))

(event EventPCStopTimer
  (bind _asw_hold_to_activate (Utilities|Casting|CastToW_HoldToActivate (Variables|Default|GetmyWidget)))
  (Default|EndTimer _asw_hold_to_activate))

(event EventVerifNbrSteleActivated
  (params (Stele :type Actor%20Object%20Reference))
  (bind _asbp_steles_mother (Utilities|Casting|CastToBP_StelesMother Stele))
  (Default|VerifNbrOfSteleActivated _asbp_steles_mother))

(fn ConstructionScript)