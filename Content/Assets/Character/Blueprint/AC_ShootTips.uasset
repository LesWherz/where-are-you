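; Actor component on BP_PlayerProto that shows a tooltip widget when the player's resize laser line rests on a specific object type.
; Each tick, only for player character 0, a line trace between the laser's start and end points sets whether a tip is needed.
; A delay timer accumulates before W_ToolTips is added through the player's client widget functions; losing the hit removes it and resets the timer.
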(event EventBeginPlay)

(event EventTick
  (params (DeltaSeconds :type Float%20%28single-precision%29))
  (bind _owner (CallFunction|Owner))
  (if (== (Components|GetOwner) (Game|GetPlayerCharacter 0))
    (bind _outhit (Collision|LineTraceForObjects (Variables|/Game/Assets/Character/Blueprint/BP_PlayerProto.BP_PlayerProto_C|GetResizeLaserStartPoint _owner) (Variables|/Game/Assets/Character/Blueprint/BP_PlayerProto.BP_PlayerProto_C|GetResizeLaserEndPoint _owner) (Utilities|Array|MakeArray "ObjectTypeQuery12") false 0 "None" true "(R=1.000000,G=0.000000,B=0.704562,A=1.000000)" "(R=0.000000,G=1.000000,B=0.000000,A=1.000000)" 1.0))
    (Utilities|FlowControl|Sequence
      (:then_0
        (if (.bblockinghit _outhit)
          (if (not (Variables|Default|GetNeedTips))
            (Variables|Default|SetNeedTips true))
          (elif (Variables|Default|GetNeedTips)
            (Variables|Default|SetNeedTips false)
            (CallFunction|RemoveTips)
            (Variables|Default|SetCurrentDelay 0.0))))
      (:then_1
        (if (and (Variables|Default|GetNeedTips) (not (Variables|Default|GetTipsIsDiplay)))
          (if (Utilities|DelayIsWaiting)
            (CallFunction|DisplayTips)
            (else
              (Variables|Default|SetCurrentDelay (+ (Variables|Default|GetCurrentDelay) DeltaSeconds)))))))))

(fn Owner
  (return (.AsBP%20Player%20Proto (Utilities|Casting|CastToBP_PlayerProto (Components|GetOwner)))))

(fn DisplayTips
  (bind _asbp_player_proto (Utilities|Casting|CastToBP_PlayerProto (Components|GetOwner)))
  (Default|ClientAddWidgetbyClass _asbp_player_proto "/Game/Assets/UI/Widgets/W_ToolTips.W_ToolTips_C")
  (Variables|Default|SetTipsIsDiplay true))

(fn RemoveTips
  (bind _asbp_player_proto (Utilities|Casting|CastToBP_PlayerProto (Components|GetOwner)))
  (Default|ClientRemoveAllWidgetbyClass _asbp_player_proto "/Game/Assets/UI/Widgets/W_ToolTips.W_ToolTips_C")
  (Variables|Default|SetTipsIsDiplay false))