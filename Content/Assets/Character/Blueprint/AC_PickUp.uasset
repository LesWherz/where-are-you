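; Player actor component that lets BP_PlayerProto pick up, carry, drop and use items on interactable objects.
; OnCharacterInteract line-traces along the owner's laser points to pick up when empty-handed, or interact or drop when holding.
; Actions propagate through Server then All events into interface-driven functions that notify objects, with animation triggers on pickup and drop.
; While PhysicallyLocked, Tick snaps the held item in front of the owner.
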(event EventBeginPlay
  (bind _asbp_player_proto (Utilities|Casting|CastToBP_PlayerProto (Components|GetOwner)))
  (Variables|Default|SetOwner _asbp_player_proto))

(event EventTick
  (params (DeltaSeconds :type Float%20%28single-precision%29))
  (if (Variables|Default|GetPhysicallyLocked)
    (bind _hasitempickedup (CallFunction|HasItemPickedUp))
    (if _hasitempickedup
      (CallFunction|AtachPickedUpObject))))

(event Custom|OnPickUpObject
  (params (pickableObject :type I%20Pickable%20Object%20Interface))
  (Default|PlayAnimationTrigger (Variables|Default|GetOwner) "NewEnumerator13"))

(event Custom|OnDropObject
  (params (pickableObject :type I%20Pickable%20Object%20Interface))
  (Default|PlayAnimationTrigger (Variables|Default|GetOwner) "NewEnumerator14"))

(event Custom|OnInteractWith
  (params (pickableObject :type I%20Pickable%20Object%20Interface) (interactableObject :type I%20Interactable%20Object%20Interface)))

(event Custom|Drop_Server
  (params (fromInteraction :type Boolean))
  ;[1 1 1] Events propagation
  (CallFunction|DropAll fromInteraction))

(event Custom|PickUp_All
  (params (toPickup :type Pickable%20Object%20Base%20Object%20Reference))
  ;[1 1 1] Events propagation
  (bind _returnvalue (Class|IPickableObject|GetIPickableObject toPickup))
  (CallFunction|PickUp _returnvalue))

(event Custom|PickUp_Server
  (params (toPickup :type Pickable%20Object%20Base%20Object%20Reference))
  ;[1 1 1] Events propagation
  (CallFunction|PickUpAll toPickup))

(event Custom|Drop_All
  (params (fromInteraction :type Boolean))
  ;[1 1 1] Events propagation
  (CallFunction|Drop fromInteraction))

(event Custom|InteractWith_Server
  (params (interactedObject :type Interactable%20Object%20Base%20Object%20Reference))
  ;[1 1 1] Events propagation
  (CallFunction|InteractwithAll interactedObject))

(event Custom|InteractWith_All
  (params (interactedObject :type Interactable%20Object%20Base%20Object%20Reference))
  ;[1 1 1] Events propagation
  (bind _returnvalue (Class|IInteractableObject|GetIInteractableObject interactedObject))
  (CallFunction|Interactwith _returnvalue))

(fn PickUp
  (params (objectToPickUp :type I%20Pickable%20Object%20Interface))
  (bind _returnvalue (Class|IPickableObject|IsPickedUp objectToPickUp))
  (if _returnvalue
    (Development|PrintString "Can't PickUp : this item is allready picked up")
    (else
      (Class|IPickableObject|OnPickedUp objectToPickUp (Variables|Default|GetOwner))
      (Variables|Default|SetPhysicallyLocked true)
      (bind _output_get (Variables|Default|SetPickedUpObject objectToPickUp))
      (CallFunction|OnPickUpObject _output_get)
      (return))))

(fn Drop
  (params (fromInteraction :type Boolean))
  (bind _hasitempickedup (CallFunction|HasItemPickedUp))
  (if _hasitempickedup
    (Class|IPickableObject|OnDropped (Variables|Default|GetPickedUpObject) (Variables|Default|GetOwner) fromInteraction)
    (CallFunction|OnDropObject (Variables|Default|GetPickedUpObject))
    (Variables|Default|SetPickedUpObject 0)
    (return)))

(fn AtachPickedUpObject
  (bind _returnvalue (Components|GetOwner))
  (bind _pickedupobject (Variables|Default|GetPickedUpObject))
  (Utilities|IsValid (Utilities|ToObject(Interface) _pickedupobject)
    (:Is%20Valid
      (bind _returnvalue_2 (Class|IPickableObject|GetTargetActor _pickedupobject))
      ;[1 1 1] Snap logic, should be modified tu be more modular
      (Transformation|SetActorLocation _returnvalue_2 (+ (Transformation|GetActorLocation _returnvalue) (* (Transformation|GetActorForwardVector _returnvalue) 2e+02)) false false)
      (Transformation|SetActorRotation _returnvalue_2 (Transformation|GetActorRotation _returnvalue))
      (return))))

(fn TryPickUp
  (params (rayStartPostition :type Vector) (rayEndPosition :type Vector))
  (bind (_outhit _returnvalue) (Collision|LineTraceForObjects rayStartPostition rayEndPosition (Utilities|Array|MakeArray "ObjectTypeQuery10") false 0 "ForDuration" true "(R=1.000000,G=0.000000,B=0.938686,A=1.000000)"))
  (if _returnvalue
    (bind _asipickable_object (Utilities|Casting|CastToIPickableObject (.HitActor (Collision|BreakHitResult _outhit)))
      (:then
        (return true _asipickable_object))
      (:CastFailed
        _)))
  (return false 0))

(fn HasItemPickedUp
  (Utilities|IsValid (Utilities|ToObject(Interface) (Variables|Default|GetPickedUpObject))
    (:Is%20Valid
      (return true))
    (:Is%20Not%20Valid
      (return false))))

(fn OnCharacterInteract
  (bind _owner (Variables|Default|GetOwner))
  (bind _owner_2 (Variables|Default|GetOwner))
  (bind _hasitempickedup (CallFunction|HasItemPickedUp))
  (if _hasitempickedup
    (bind (_success _interactableobject) (CallFunction|TryInteract (Variables|/Game/Assets/Character/Blueprint/BP_PlayerProto.BP_PlayerProto_C|GetResizeLaserStartPoint _owner_2) (Variables|/Game/Assets/Character/Blueprint/BP_PlayerProto.BP_PlayerProto_C|GetResizeLaserEndPoint _owner_2)))
    (if _success
      (bind _asinteractable_object_base (Utilities|Casting|CastToInteractableObjectBase _interactableobject))
      (CallFunction|InteractwithServer _asinteractable_object_base)
      (return)
      (else
        (CallFunction|DropServer false)
        (return)))
    (else
      (bind (_success_2 _pickedupobject) (CallFunction|TryPickUp (Variables|/Game/Assets/Character/Blueprint/BP_PlayerProto.BP_PlayerProto_C|GetResizeLaserStartPoint _owner) (Variables|/Game/Assets/Character/Blueprint/BP_PlayerProto.BP_PlayerProto_C|GetResizeLaserEndPoint _owner)))
      (if _success_2
        (bind _aspickable_object_base (Utilities|Casting|CastToPickableObjectBase _pickedupobject))
        (CallFunction|PickUpServer _aspickable_object_base)
        (return)))))

(fn TryInteract
  (params (rayStartPostition :type Vector) (rayEndPosition :type Vector))
  (bind _outhit (Collision|LineTraceForObjects rayStartPostition rayEndPosition (Utilities|Array|MakeArray "ObjectTypeQuery13") false 0 "ForDuration" true "(R=1.000000,G=0.000000,B=0.938686,A=1.000000)"))
  (if true
    (bind _asiinteractable_object (Utilities|Casting|CastToIInteractableObject (.HitActor (Collision|BreakHitResult _outhit)))
      (:then
        (return true _asiinteractable_object))
      (:CastFailed
        _)))
  (return false 0))

(fn Interactwith
  (params (interactableObject :type I%20Interactable%20Object%20Interface))
  (bind _pickedupobject (Variables|Default|GetPickedUpObject))
  (bind _hasitempickedup (CallFunction|HasItemPickedUp))
  (if _hasitempickedup
    (CallFunction|OnInteractwith _pickedupobject interactableObject)
    (Variables|Default|SetPhysicallyLocked false)
    (LocalVariables|SetDroppedObject _pickedupobject)
    (CallFunction|DropServer true)
    (Class|IPickableObject|OnInteracted (LocalVariables|GetDroppedObject) interactableObject)
    (else
      (Development|PrintString "Can't InteractWith : you don't have an item picked up" true true "(R=1.000000,G=0.000000,B=0.093894,A=1.000000)"))))