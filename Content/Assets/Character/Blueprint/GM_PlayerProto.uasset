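; Game mode for a two-player party that holds players on a waiting screen until both have joined.
; PostLogin and PlayerLeave update the player list and count, then tell each PC_PlayerProto to start or stop waiting.
; ChoosePlayerStart hands out PlayerStarts in sequence through an incrementing index, falling back to the first when exhausted.
; It also issues incrementing resizable IDs and exposes the player count.
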(event Custom|isEverybodyThere
  ;[1 0.9331 0] Waiting screen for other player to join
  (if (== (Variables|Default|GetnumberOfPlayer) 2)
    (for _array_element (Variables|Default|GetList_Player)
      (Default|StopWaitSecondPlayer _array_element))
    (else
      (for _array_element_2 (Variables|Default|GetList_Player)
        (Default|WaitSecondPlayer _array_element_2)))))

(event Custom|PlayerLeave
  (params (ItemToFind :type PC%20Player%20Proto%20Object%20Reference%20%28by%20ref%29))
  (bind _list_player (Variables|Default|GetList_Player))
  ;[1 0.9388 0.05874] player leave
  (Utilities|Array|RemoveIndex _list_player (Utilities|Array|FindItem _list_player ItemToFind))
  (Math|Integer|DecrementInt (Variables|Default|GetnumberOfPlayer)
    (:%20%20
      (CallFunction|IsEverybodyThere))))

(event EventPostLogin
  (params (NewPlayer :type Player%20Controller%20Object%20Reference))
  ;[1 1 1] Player Join Party
  (bind _aspc_player_proto (Utilities|Casting|CastToPC_PlayerProto NewPlayer))
  (Utilities|Array|AddUnique (Variables|Default|GetList_Player) _aspc_player_proto)
  (Math|Integer|IncrementInt (Variables|Default|GetnumberOfPlayer)
    (:%20%20
      (CallFunction|IsEverybodyThere))))

(fn ConstructionScript)

(fn ChoosePlayerStart
  (params (Player :type Controller%20Object%20Reference))
  (bind _spawnincrement_dirty (Variables|Default|GetSpawnIncrement_Dirty))
  ;[1 1 1] Spawn des joueurs sur des PlayerStart diférents
  (bind _outactors (Actor|GetAllActorsOfClass "/Script/Engine.PlayerStart"))
  (if (Utilities|Array|IsValidIndex _outactors _spawnincrement_dirty)
    (bind _output_get (LocalVariables|SetPlayerStart (Utilities|Array|Get(acopy) _outactors _spawnincrement_dirty)))
    (Math|Integer|IncrementInt (Variables|Default|GetSpawnIncrement_Dirty)
      (:%20%20
        (return _output_get)))
    (else
      (return (Utilities|Array|Get(acopy) _outactors)))))

(fn GetResizableId
  (bind _result (Math|Integer|IncrementInt (Variables|Default|GetResizableId))
    (:%20%20
      (bind _output_get (Variables|Default|SetResizableId _result))
      (return _output_get))))

(fn GetNumberOfPlayer
  (return (Variables|Default|GetnumberOfPlayer)))