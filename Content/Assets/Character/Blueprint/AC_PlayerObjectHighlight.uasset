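; Player actor component that highlights the interactive object under the gun laser by showing its ShrunkedBoxCollision.
; While the player's size state is Normal, Tick runs an object-type line trace between the laser's start and end points.
; A hit BP_InteractiveObjects is cached as AimedResizableObject and its box is unhidden.
; The previous box is hidden when the hit actor changes or the trace misses.
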(event EventBeginPlay
  ;[1 1 1] Get the player owner
  (bind _asbp_player_proto (Utilities|Casting|CastToBP_PlayerProto (Components|GetOwner self)))
  (Variables|Default|SetPlayerOwner _asbp_player_proto))

(event EventTick
  (params (DeltaSeconds :type Float%20%28single-precision%29))
  (bind _aimedresizableobject (Variables|Default|GetAimedResizableObject))
  (bind _playerowner (Variables|Default|GetPlayerOwner))
  ;[1 1 1] Shrunked Object Highlight
  (if (Utilities|Enum|Equal(Enum) (Variables|/Game/Assets/Character/Blueprint/AC_ResizePlayer.AC_ResizePlayer_C|GetPlayerSizeState (Variables|/Game/Assets/Character/Blueprint/BP_PlayerProto.BP_PlayerProto_C|GetAC_ResizePlayer (Variables|Default|GetPlayerOwner))) "Normal")
    (bind _outhit (Collision|LineTraceForObjects (Variables|/Game/Assets/Character/Blueprint/BP_PlayerProto.BP_PlayerProto_C|GetGunLaserStartPoint _playerowner) (Variables|/Game/Assets/Character/Blueprint/BP_PlayerProto.BP_PlayerProto_C|GetGunLaserEndPoint _playerowner) (Utilities|Array|MakeArray "ObjectTypeQuery11") false 0 "None" true "(R=1.000000,G=0.000000,B=0.000000,A=1.000000)" "(R=0.000000,G=1.000000,B=0.000000,A=1.000000)" 1.0))
    (if (.bblockinghit _outhit)
      (if (and (!= (.hitactor _outhit) _aimedresizableobject) (Utilities|IsValid _aimedresizableobject))
        (Utilities|FlowControl|Sequence
          (:then_0
            (CallFunction|TryStopAimingCurrentObject :!label _label))
          (:then_1
            (bind _asbp_interactive_objects (Utilities|Casting|CastToBP_InteractiveObjects (.hitactor _outhit) :!label _label_2))
            (CallFunction|StartAimingObject _asbp_interactive_objects)))
        (else
          (goto _label_2)))
      (else
        (goto _label)))))

(fn StartAimingObject
  (params (ObjectToAim :type BP%20Interactive%20Objects%20Object%20Reference))
  (Variables|Default|SetAimedResizableObject ObjectToAim)
  (Development|SetHiddeninGame (Variables|/Game/Blueprints/BP_InteractibleObject/BP_InteractiveObjects.BP_InteractiveObjects_C|GetShrunkedBoxCollision (Variables|Default|GetAimedResizableObject)) false false))

(fn TryStopAimingCurrentObject
  (Utilities|IsValid (Variables|Default|GetAimedResizableObject)
    (:Is%20Valid
      (Development|SetHiddeninGame (Variables|/Game/Blueprints/BP_InteractibleObject/BP_InteractiveObjects.BP_InteractiveObjects_C|GetShrunkedBoxCollision (Variables|Default|GetAimedResizableObject)) true false)
      (Variables|Default|SetAimedResizableObject 0))))