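; BP_PilierGen is a procedural prop Blueprint that generates a row of pillar static meshes along its local X axis.
; The Construction Script adds one component per NumberOfPillars, with a shared Scale and fixed Y and Z offsets.
; Each pillar sits Length divided by the count beyond the previous one, chained through PreviousSM; with no valid predecessor, X is zero.
; The event graph has no runtime logic.
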(event EventBeginPlay)

(fn ConstructionScript
  (bind _number_of_pillars (Variables|Default|GetNumber%20of%20Pillars))
  (for _index (range 1 _number_of_pillars)
    (bind _returnvalue (AddComponent|AddStaticMeshComponent false (Math|Transform|MakeTransform (Math|Vector|MakeVector (select (Utilities|IsValid (Variables|Default|GetPreviousSM)) (+ (/ (Variables|Default|GetLength) (Math|Conversions|ToFloat(Integer) _number_of_pillars)) (.x (Variables|/Script/Engine.SceneComponent|GetRelativeLocation (Variables|Default|GetPreviousSM)))) 0.0) 9e+01 -2.5) "0, 0, 0" (Variables|Default|GetScale))))
    (Variables|Default|SetPreviousSM _returnvalue)))