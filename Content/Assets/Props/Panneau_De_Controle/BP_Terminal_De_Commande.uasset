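; BP_Terminal_De_Commande is a control panel prop intended to show or hide help text when the player overlaps its Box.
; The begin-overlap event only checks for the local BP_PlayerProto and does nothing further; BeginPlay, end overlap and the construction script are empty.
; Disconnected nodes hold the unused logic: toggling visibility, playing a display beep, and setting editable text and light intensity.
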(event OnComponentBeginOverlap(Box)
  (params (OverlappedComponent :type Primitive%20Component%20Object%20Reference) (OtherActor :type Actor%20Object%20Reference) (OtherComp :type Primitive%20Component%20Object%20Reference) (OtherBodyIndex :type Integer) (bFromSweep :type Boolean) (SweepResult :type Hit%20Result%20Structure%20%28by%20ref%29))
  ;[1 1 1] affiche ou masque le texte d'aide
  (bind _asbp_player_proto (Utilities|Casting|CastToBP_PlayerProto OtherActor))
  (if (== _asbp_player_proto (.AsBP%20Player%20Proto (Utilities|Casting|CastToBP_PlayerProto (Game|GetPlayerCharacter 0))))
    _))

(event OnComponentEndOverlap(Box)
  (params (OverlappedComponent :type Primitive%20Component%20Object%20Reference) (OtherActor :type Actor%20Object%20Reference) (OtherComp :type Primitive%20Component%20Object%20Reference) (OtherBodyIndex :type Integer))
  ;[1 1 1] affiche ou masque le texte d'aide
)

(event EventBeginPlay
  ;[1 1 1] affiche ou masque le texte d'aide
)

(fn ConstructionScript
  ;[1 1 1] Set le texte au démarrage + modifiable dans le world
)