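; BP_LightBase is a base Blueprint for light props that can be toggled with on and off sounds.
; The construction script gathers all of its light components, and BeginPlay creates a dynamic material instance from the static mesh's first material slot.
; ToggleLights passes those lights, the lamp material and the two sounds to ToggleLight, which is defined outside these graphs.
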(event EventBeginPlay
  (bind _staticmesh (Variables|Default|GetStaticMesh))
  (bind _returnvalue (Rendering|Material|CreateDynamicMaterialInstance _staticmesh 0 (Rendering|Material|GetMaterial _staticmesh 0) "None" :!class /Script/Engine.PrimitiveComponent))
  (Variables|Default|SetLampMaterial _returnvalue))

(event EventToggleLights
  (params (Sound%20ON :type Sound%20Cue%20Object%20Reference) (Sound%20OFF :type Sound%20Cue%20Object%20Reference))
  (CallFunction|ToggleLight Sound%20ON Sound%20OFF (Variables|Default|GetLights) (Variables|Default|GetLampMaterial)))

(fn ConstructionScript
  (Variables|Default|SetLights (Actor|GetComponentsByClass "/Script/Engine.LightComponent")))