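; BP_Ampoule1 is a light bulb prop with configurable color and intensity and an optional flicker.
; The construction script creates a dynamic material instance for the bulb mesh and sets the point light and emissive tint and force from Color and Intensity.
; When Flicker is enabled, a timeline started at BeginPlay scales light intensity and emissive force together, using a stronger emissive ratio than the static setup.
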(event EventBeginPlay
  (if (Variables|Default|GetFlicker)
    (bind _newtrack_0 (Timeline|Timeline_0 PlayFromStart)
      (:Update
        (Rendering|Components|Light|SetIntensity (Variables|Default|GetPointLight) (* (Variables|Default|GetIntensity) _newtrack_0))
        (Rendering|Material|SetScalarParameterValue (Variables|Default|GetMat) "Emissive Force" (/ (* (Variables|Default|GetIntensity) _newtrack_0) 2e+02) :!class /Script/Engine.MaterialInstanceDynamic)))))

(fn ConstructionScript
  (bind _color (Variables|Default|GetColor))
  (Rendering|Components|Light|SetIntensity (Variables|Default|GetPointLight) (Variables|Default|GetIntensity))
  (bind _returnvalue (Rendering|Material|CreateDynamicMaterialInstance "/Game/Assets/Props/Ampoule_01/MI_Ampoule01.MI_Ampoule01" "None" "None" :!class /Script/Engine.KismetMaterialLibrary))
  (Variables|Default|SetMat _returnvalue)
  (for _index (range 0 2)
    (Rendering|Material|SetMaterial (Variables|Default|GetSM_Ampoule_01) _index _returnvalue))
  (Rendering|Components|Light|SetLightColor (Variables|Default|GetPointLight) (Math|Conversions|ToLinearColor(Color) _color) true)
  (Rendering|Material|SetVectorParameterValue _returnvalue "ㅤㅤㅤ- Emissive Tint" (Math|Conversions|ToLinearColor(Color) _color) :!class /Script/Engine.MaterialInstanceDynamic)
  (Rendering|Material|SetScalarParameterValue (Variables|Default|GetMat) "Emissive Force" (/ (Variables|Default|GetIntensity) 1e+03) :!class /Script/Engine.MaterialInstanceDynamic))