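; Plant prop Blueprint with a point light and a decal, configured entirely in the Construction Script with no active event logic.
; The script applies the exposed intensity and color to the light and places the decal at a fixed offset below the origin.
; When AUTOROTATELP is enabled, it also randomizes actor scale, slight tilt, full yaw and decal size for placement variety, re-rolling on each construction run.
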(event EventBeginPlay)

(event Collision|EventActorBeginOverlap
  (params (OtherActor :type Actor%20Object%20Reference)))

(event EventTick
  (params (DeltaSeconds :type Float%20%28single-precision%29)))

(fn ConstructionScript
  (bind _returnvalue (Math|Random|RandomFloatinRange 0.0 5.0))
  ;[1 1 1] Set intensité de la light et sa couleur lors du play
  (Rendering|Components|Light|SetIntensity (Variables|Default|GetPointLight) (Variables|Default|GetLight_Intensity))
  (Rendering|Components|Light|SetLightColor (Variables|Default|GetPointLight) (Variables|Default|GetNew%20Light%20Color) true)
  (Transformation|SetRelativeLocation (Variables|Default|GetDecal) "0, 0,-35.000000" false false)
  (if (Variables|Default|GetAUTO%20ROTATE%20LP)
    (Transformation|SetActorScale3D (Math|Conversions|ToVector(Float) (Math|Random|RandomFloatinRange 0.95 1.2)))
    (Transformation|SetActorRotation (Math|Rotator|MakeRotator _returnvalue _returnvalue (Math|Random|RandomFloatinRange 0.0 3.6e+02)))
    (Transformation|SetRelativeScale3D (Variables|Default|GetDecal) (Math|Conversions|ToVector(Float) (Math|Random|RandomFloatinRange 0.4 0.5)))))