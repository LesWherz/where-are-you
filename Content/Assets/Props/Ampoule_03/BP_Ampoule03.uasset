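; Light bulb prop Blueprint that pairs a mesh with a rect light, with configurable color, intensity and optional flicker.
; The construction script sets the light's intensity and color and creates a dynamic material instance tinted to match.
; When Flicker is enabled, BeginPlay starts a timeline whose track scales both light intensity and emissive force, keeping the glow in sync with the light.
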(event EventBeginPlay
  (if (Variables|Default|GetFlicker)
    (bind _newtrack_0 (Timeline|Timeline_0 PlayFromStart)
      (:Update
        (Rendering|Components|Light|SetIntensity (Variables|Default|GetRectLight) (* (Variables|Default|GetIntensity) _newtrack_0))
        (Rendering|Material|SetScalarParameterValue (Variables|Default|GetMat) "Emissive Force" (* _newtrack_0 5.0) :!class /Script/Engine.MaterialInstanceDynamic)))))

(fn ConstructionScript
  (bind _color (Variables|Default|GetColor))
  (Rendering|Components|Light|SetIntensity (Variables|Default|GetRectLight) (Variables|Default|GetIntensity))
  (bind _returnvalue (Rendering|Material|CreateDynamicMaterialInstance "/Game/Assets/Props/Ampoule_03/MI_Ampoule03.MI_Ampoule03" "None" "None" :!class /Script/Engine.KismetMaterialLibrary))
  (Variables|Default|SetMat _returnvalue)
  (Rendering|Material|SetMaterial (Variables|Default|GetSM_Ampoule_03) 0 _returnvalue)
  (Rendering|Components|Light|SetLightColor (Variables|Default|GetRectLight) (Math|Conversions|ToLinearColor(Color) _color) true)
  (Rendering|Material|SetVectorParameterValue _returnvalue "ㅤㅤㅤ- Emissive Tint" (Math|Conversions|ToLinearColor(Color) _color) :!class /Script/Engine.MaterialInstanceDynamic))